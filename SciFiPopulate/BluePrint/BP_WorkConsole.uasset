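; BP_WorkConsole is a modular sci-fi work console prop built from top, middle and bottom static mesh components, varied at placement in the editor.
; The construction script checks IsRandom to either pick each part from its mesh array with a random stream or use per-part variation indices.
; The manual indices are clamped to the array bounds, and the event graph holds no active logic.
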(event EventBeginPlay)

(event EventActorBeginOverlap
  (params (OtherActor :type Actor%20Object%20Reference)))

(event EventTick
  (params (DeltaSeconds :type Float%20%28single-precision%29)))

(fn ConstructionScript
  (if (Variables|Random|GetisRandom) ; Should meshes be random \npopulated or picked from the lists
    (|Randommeshselectionmethod)
    (else
      (|Variationusingmethod))))