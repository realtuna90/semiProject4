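; BP_GasRoom is a gas hazard volume that deals escalating poison damage to the player's MotionControllerPawn while it is inside.
; Box overlap events toggle the damage flag, and leaving also resets the toxicity.
; While the flag is set, Tick runs through a Delay that paces each step, raising the toxic amount and passing it to PoisonDamage on the pawn cached at BeginPlay.
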(event OnComponentBeginOverlap(Box)
  (params (OverlappedComponent :type Primitive%20Component%20Object%20Reference) (OtherActor :type Actor%20Object%20Reference) (OtherComp :type Primitive%20Component%20Object%20Reference) (OtherBodyIndex :type Integer) (bFromSweep :type Boolean) (SweepResult :type Hit%20Result%20Structure%20%28by%20ref%29))
  (Utilities|Casting|CastToMotionControllerPawn OtherActor)
  (Variables|Default|SetonDamage true))

(event OnComponentEndOverlap(Box)
  (params (OverlappedComponent :type Primitive%20Component%20Object%20Reference) (OtherActor :type Actor%20Object%20Reference) (OtherComp :type Primitive%20Component%20Object%20Reference) (OtherBodyIndex :type Integer))
  (Utilities|Casting|CastToMotionControllerPawn OtherActor)
  (Variables|Default|SetonDamage false)
  (Variables|Default|SetToxicAmount 0))

(event EventBeginPlay
  (bind _asmotion_controller_pawn (Utilities|Casting|CastToMotionControllerPawn (Game|Player|GetPlayerPawn 0)))
  (Variables|Default|SetPlayer _asmotion_controller_pawn))

(event EventTick
  (params (DeltaSeconds :type Float%20%28single-precision%29))
  (if (Variables|Default|GetonDamage)
    (Utilities|FlowControl|Delay (Variables|Default|GetIncreaseTime))
    (bind _output_get (Variables|Default|SetToxicAmount (+ (Variables|Default|GetToxicAmount) (Variables|Default|GetIncreaseAmount))))
    (Default|PoisonDamage (Variables|Default|GetPlayer) _output_get)))

(fn ConstructionScript)