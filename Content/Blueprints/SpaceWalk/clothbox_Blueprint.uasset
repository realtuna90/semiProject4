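; Clothes box trigger for the space-walk sequence, active only while the VR game mode's Level is at one specific stage.
; Overlapping its Box calls the game mode's LoadLevel to load "outside_3" and unload "SemiLevel_open_2".
; Tick polls the same stage and, through a DoOnce, plays two delayed TTS announcements, the second urging an emergency change of clothes.
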(event OnComponentBeginOverlap(Box)
  (params (OverlappedComponent :type Primitive%20Component%20Object%20Reference) (OtherActor :type Actor%20Object%20Reference) (OtherComp :type Primitive%20Component%20Object%20Reference) (OtherBodyIndex :type Integer) (bFromSweep :type Boolean) (SweepResult :type Hit%20Result%20Structure%20%28by%20ref%29))
  (bind _asvrgame_mode (Utilities|Casting|CastToVRGameMode (Game|GetGameMode)))
  (if (Utilities|Enum|Equal(Enum) (Variables|/Game/Blueprints/VRGameMode.VRGameMode_C|Getlevel _asvrgame_mode) "NewEnumerator1")
    (Default|LoadLevel _asvrgame_mode "outside_3" "SemiLevel_open_2")))

(event EventTick
  (params (DeltaSeconds :type Float%20%28single-precision%29))
  (bind _asvrgame_mode (Utilities|Casting|CastToVRGameMode (Game|GetGameMode)))
  (if (Utilities|Enum|Equal(Enum) (Variables|/Game/Blueprints/VRGameMode.VRGameMode_C|Getlevel _asvrgame_mode) "NewEnumerator1")
    (Utilities|FlowControl|DoOnce false
      (:Completed
        (Utilities|FlowControl|Delay 2.0)
        (Audio|PlaySound2D "/Game/4Sound/엔진실외TTS.엔진실외TTS" 2.0 1.0 0.0 0 0)
        (Utilities|FlowControl|Delay 3.7)
        (Audio|PlaySound2D "/Game/4Sound/긴급환복바람TTS.긴급환복바람TTS" 2.0 1.0 0.0 0 0)))))

(fn ConstructionScript)