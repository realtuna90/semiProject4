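; BP_PullingLever is a VR lever that a motion controller grabs and slides along its local Z axis.
; While dragged with ResettingPosition true, Tick converts the controller's GrabSphere position into actor space and clamps the lever's Z between MinPitch and MaxPitch.
; Drop plays a timeline that lerps the lever back to InitialLeverLocation, setting ResettingPosition until it finishes.
; Controller overlap on LeverBall toggles a highlight material and an overlap flag.
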(event OnComponentBeginOverlap(LeverBall)
  (params (OverlappedComponent :type Primitive%20Component%20Object%20Reference) (OtherActor :type Actor%20Object%20Reference) (OtherComp :type Primitive%20Component%20Object%20Reference) (OtherBodyIndex :type Integer) (bFromSweep :type Boolean) (SweepResult :type Hit%20Result%20Structure%20%28by%20ref%29))
  (Utilities|Casting|CastToBP_MotionController OtherActor)
  (Rendering|Material|SetMaterial (Variables|Default|GetLeverBall) 0 "/Game/VirtualReality/Materials/BasicHighlightMaterial.BasicHighlightMaterial")
  (Variables|Default|SetOnoverlap true))

(event OnComponentEndOverlap(LeverBall)
  (params (OverlappedComponent :type Primitive%20Component%20Object%20Reference) (OtherActor :type Actor%20Object%20Reference) (OtherComp :type Primitive%20Component%20Object%20Reference) (OtherBodyIndex :type Integer))
  (Utilities|Casting|CastToBP_MotionController OtherActor)
  (Rendering|Material|SetMaterial (Variables|Default|GetLeverBall) 0 "/Game/VirtualReality/Materials/BasicCubeMaterial.BasicCubeMaterial")
  (Variables|Default|SetOnoverlap false))

(event EventTick
  (params (DeltaSeconds :type Float%20%28single-precision%29))
  (Utilities|IsValid (Variables|Default|GetBPMotionController)
    (:Is%20Valid
      (if (Variables|Default|GetIsdrag)
        (if (Variables|Default|GetResettingPosition)
          (Transformation|SetRelativeLocation (Variables|Default|GetLever) (Math|Vector|MakeVector 0.0 0.0 (Math|Float|Clamp(Float) (.z (Math|Transform|InverseTransformLocation (Transformation|GetActorTransform) (Transformation|GetWorldLocation (Variables|/Game/Blueprints/BP_MotionController.BP_MotionController_C|GetGrabSphere (Variables|Default|GetBPMotionController))))) (Variables|Default|GetMinPitch) (Variables|Default|GetMaxPitch))) false false))))))

(event EventPickup
  (params (AttachTo :type BP%20Motion%20Controller%20Object%20Reference))
  (Variables|Default|SetIsdrag true)
  (Variables|Default|SetBPMotionController AttachTo))

(event EventDrop
  (Variables|Default|SetIsdrag false)
  (Variables|Default|SetResettingPosition true)
  (Variables|Default|SetInterpLeverLocation (Variables|/Script/Engine.SceneComponent|GetRelativeLocation (Variables|Default|GetLever)))
  (bind _새_트랙_0 (Timeline|타임라인_0 PlayFromStart)
    (:Update
      (Transformation|SetRelativeLocation (Variables|Default|GetLever) (Math|Vector|MakeVector 0.0 0.0 (.z (Math|Vector|Lerp(Vector) (Variables|Default|GetInterpLeverLocation) (Variables|Default|GetInitialLeverLocation) _새_트랙_0))) false false))
    (:Finished
      (Variables|Default|SetResettingPosition false))))

(fn ConstructionScript)