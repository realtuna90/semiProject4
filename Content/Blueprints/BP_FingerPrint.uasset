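; BP_FingerPrint is a fingerprint scanner that signals a door to open when a VR motion controller touches it.
; Overlap events on its Box component respond only to BP_MotionController, calling OpenDoor and turning the screen material green.
; When the overlap ends, the screen turns blue and CloseDoor is called after a short delay.
; The door logic itself lives outside this Blueprint.
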(event OnComponentBeginOverlap(Box)
  (params (OverlappedComponent :type Primitive%20Component%20Object%20Reference) (OtherActor :type Actor%20Object%20Reference) (OtherComp :type Primitive%20Component%20Object%20Reference) (OtherBodyIndex :type Integer) (bFromSweep :type Boolean) (SweepResult :type Hit%20Result%20Structure%20%28by%20ref%29))
  (Utilities|IsValid OverlappedComponent
    (:Is%20Valid
      (Utilities|Casting|CastToBP_MotionController OtherActor)
      (Default|CallOpenDoor)
      (Rendering|Material|SetMaterial (Variables|Default|GetFingerPrint) 1 "/Game/2Materials/Screen_Green.Screen_Green"))))

(event OnComponentEndOverlap(Box)
  (params (OverlappedComponent :type Primitive%20Component%20Object%20Reference) (OtherActor :type Actor%20Object%20Reference) (OtherComp :type Primitive%20Component%20Object%20Reference) (OtherBodyIndex :type Integer))
  (Utilities|IsValid OverlappedComponent
    (:Is%20Valid
      (Utilities|Casting|CastToBP_MotionController OtherActor)
      (Rendering|Material|SetMaterial (Variables|Default|GetFingerPrint) 1 "/Game/2Materials/Screen_Blue.Screen_Blue")
      (Utilities|FlowControl|Delay 3.0)
      (Default|CallCloseDoor))))

(fn ConstructionScript)