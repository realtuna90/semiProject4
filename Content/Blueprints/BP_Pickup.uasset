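; BP_Pickup is a grabbable VR actor that motion controllers can pick up and drop.
; Pickup, called by BP_MotionController, disables mesh physics and attaches the root to the given component, keeping world transform.
; Drop re-enables physics and detaches it in place.
; On BeginPlay, if VRGameMode's Level matches one specific stage, it also passes BP_GasManager's current Phase to the game mode's CallOnChangePhase.
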(event EventBeginPlay
  (bind _asvrgame_mode (Utilities|Casting|CastToVRGameMode (Game|GetGameMode)))
  (if (Utilities|Enum|Equal(Enum) (Variables|/Game/Blueprints/VRGameMode.VRGameMode_C|Getlevel _asvrgame_mode) "NewEnumerator2")
    (bind _returnvalue (Actor|GetActorOfClass "/Game/Blueprints/GasEvent/BP_GasManager.BP_GasManager_C"))
    (Default|CallOnChangePhase _asvrgame_mode (Variables|/Game/Blueprints/VRGameMode.VRGameMode_C|Getlevel _asvrgame_mode) (Variables|/Game/Blueprints/GasEvent/BP_GasManager.BP_GasManager_C|GetPhase _returnvalue))))

(event EventPickup
  (params (AttachTo :type Scene%20Component%20Object%20Reference) (MotionController :type BP%20Motion%20Controller%20Object%20Reference))
  (Physics|SetSimulatePhysics (Variables|Debug|GetStaticMeshComponent) false)
  (Transformation|AttachComponentToComponent (VehicleSound|GetRootComponent) AttachTo "None" "KeepWorld" "KeepWorld" "KeepWorld" false))

(event EventDrop
  (Physics|SetSimulatePhysics (Variables|Debug|GetStaticMeshComponent) true)
  (Transformation|DetachFromActor "KeepWorld" "KeepWorld" "KeepWorld"))

(fn ConstructionScript)