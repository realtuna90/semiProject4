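; BP_Light is a Blueprint that drives a point light which switches between a normal and a warning color.
; WarningLightOnOff flips the stored BaseColor between the Normal and Warning values, then applies it to the PointLight in sRGB.
; The construction script is empty, and nothing in the file calls the toggle itself.
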(fn ConstructionScript)

(fn WarningLightonOff
  (if (== (Variables|Default|GetBaseColor) (Variables|Default|GetNormal))
    (Variables|Default|SetBaseColor (Variables|Default|GetWarning))
    (else
      (Variables|Default|SetBaseColor (Variables|Default|GetNormal))))
  (Rendering|Components|Light|SetLightColor (Variables|Default|GetPointLight) (Variables|Default|GetBaseColor) true))