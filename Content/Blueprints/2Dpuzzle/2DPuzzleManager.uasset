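; Manager for a 2D puzzle stage in a VR game, driving its phases when the game mode switches to that stage.
; Module input and puzzle-clear events increment the phase, which per-tick Delay loops poll.
; Phase 2 fires drive-input completion, binds the puzzle and broadcasts the phase change; phase 3 only prints a clear message.
; StageClear would request a stage change but is never called.
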(event Custom|Clear
  (Math|Integer|IncrementInt (Variables|Default|GetPhase)))

(event Custom|StageClear
  ;[1 1 1] 스테이지 클리어
  (bind _asvrgame_mode (Utilities|Casting|CastToVRGameMode (Game|GetGameMode)))
  (Default|StageChange _asvrgame_mode (Variables|Default|GetstageNum)))

(event Custom|StageStart
  (params (curStage :type LevelEnum%20Enum :default "NewEnumerator4"))
  (if (Utilities|Enum|Equal(Enum) curStage (Variables|Default|GetstageNum))
    (bind _asvrgame_mode (Utilities|Casting|CastToVRGameMode (Game|GetGameMode)))
    (Default|CallOnChangePhase _asvrgame_mode (Variables|Default|GetstageNum) (Variables|Default|GetPhase))
    (Utilities|FlowControl|Sequence
      (:then_0
        (if (== (Variables|Default|GetPhase) 2) :!label _label
          (Default|CallDriveInputComplete)
          (EventDispatchers|BindEventtoPuzzleClear (Variables|Default|GetPuzzle) (delegate Custom|Clear))
          (bind _asvrgame_mode_2 (Utilities|Casting|CastToVRGameMode (Game|GetGameMode)))
          (Default|CallOnChangePhase _asvrgame_mode_2 (Variables|Default|GetstageNum) (Variables|Default|GetPhase))
          (else
            (Utilities|FlowControl|Delay 0.0)
            (goto _label))))
      (:then_1
        (if (== (Variables|Default|GetPhase) 3) :!label _label_2
          (Development|PrintString "CLEAR!!!!!!!!!!!!!!!!" true true "(R=0.000000,G=0.660000,B=1.000000,A=1.000000)" 3e+01)
          (else
            (Utilities|FlowControl|Delay 0.0)
            (goto _label_2)))))))

(event EventBeginPlay
  (bind _module (Variables|Default|GetModule))
  (bind _asvrgame_mode (Utilities|Casting|CastToVRGameMode (Game|GetGameMode)))
  (EventDispatchers|BindEventtoOnChangeStage _asvrgame_mode (delegate Custom|StageStart))
  (Utilities|IsValid _module :!label _label
    (:Is%20Valid
      (EventDispatchers|BindEventtoInput _module (delegate Custom|Clear)))
    (:Is%20Not%20Valid
      (Utilities|FlowControl|Delay 0.0)
      (goto _label))))

(fn ConstructionScript)