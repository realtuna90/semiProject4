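; BP_PuzzleNode is a 2D puzzle piece that rotates with a parent handle and casts a line toward targets.
; While the handle is controlled, the node copies, inverts or triples its rotation according to Type.
; A per-tick forward trace calls a left or right hit on BP_Target based on HandleNum.
; A spline mesh shows the line, shortened where it meets BP_2DPuzzle and extended long when nothing registers.
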(event Custom|StartControl
  (Variables|Default|SetIsControl true))

(event Custom|EndControl
  (Variables|Default|SetIsControl false))

(event EventBeginPlay
  (bind _parenthandle (Variables|디폴트|GetParentHandle))
  (EventDispatchers|BindEventtoHandleControlon _parenthandle (delegate Custom|StartControl))
  (EventDispatchers|BindEventtoHandleControlOff _parenthandle (delegate Custom|EndControl)))

(event EventTick
  (params (DeltaSeconds :type Float%20%28single-precision%29))
  (bind _startpoint (Variables|Default|GetStartPoint))
  (bind _endpoint (Variables|Default|GetEndPoint))
  (bind _startpoint_2 (Variables|Default|GetStartPoint))
  (bind _staticmesh (Variables|Default|GetStaticMesh))
  (bind _parenthandle (Variables|디폴트|GetParentHandle))
  (bind _returnvalue (Transformation|GetWorldLocation _startpoint))
  (bind _relativelocation (Variables|/Script/Engine.SceneComponent|GetRelativeLocation _startpoint_2))
  (bind _staticmesh_2 (Variables|/Game/Blueprints/2Dpuzzle/BP_Handle.BP_Handle_C|GetStaticMesh _parenthandle))
  (bind _relativerotation (Variables|/Script/Engine.SceneComponent|GetRelativeRotation _staticmesh_2))
  (Utilities|FlowControl|Sequence
    (:then_0
      (if (Variables|Default|GetIsControl)
        (switch int (Variables|Default|GetType)
          (:0
            (Transformation|SetRelativeRotation _staticmesh _relativerotation false false))
          (:1
            (Transformation|SetRelativeRotation _staticmesh (* _relativerotation -1.0) false false))
          (:2
            (Transformation|SetRelativeRotation _staticmesh (* _relativerotation 3.0) false false)))))
    (:then_1
      (Variables|Default|SetOnHit false)
      (bind _outhit (Collision|LineTraceByChannel _returnvalue (+ _returnvalue (* (Math|Vector|GetForwardVector (Variables|Default|GetStaticMesh)) 200)) "TraceTypeQuery3" false 0 "None"))
      (Utilities|FlowControl|Sequence
        (:then_0
          (bind _asbp_target (Utilities|Casting|CastToBP_Target (.HitActor (Collision|BreakHitResult _outhit))))
          (Variables|Default|SetOnHit (.bBlockingHit (Collision|BreakHitResult _outhit)))
          (if (== (Variables|Default|GetHandleNum) 1)
            (Default|CallLeftHit _asbp_target)
            (else
              (Default|CallRightHit _asbp_target))))
        (:then_1
          (Utilities|Casting|CastToBP_2DPuzzle (.HitActor (Collision|BreakHitResult _outhit)))
          (Transformation|SetWorldLocation _endpoint (.Location (Collision|BreakHitResult _outhit)) false false)
          (SplineMesh|SetEndPosition (Variables|Default|GetSplineMesh) (Variables|/Script/Engine.SceneComponent|GetRelativeLocation _endpoint) true)
          (Variables|Default|SetOnHit true))))
    (:then_2
      (if (not (Variables|Default|GetOnHit))
        (SplineMesh|SetStartandEnd (Variables|Default|GetSplineMesh) _relativelocation "0, 0, 0" (+ _relativelocation (* (Math|Vector|GetForwardVector (Variables|/Script/Engine.SceneComponent|GetRelativeRotation _startpoint_2)) 4e+03)) "0, 0, 0" true :!class /Script/Engine.SplineMeshComponent)))))

(fn ConstructionScript)