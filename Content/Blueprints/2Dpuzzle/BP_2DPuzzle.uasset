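; BP_2DPuzzle is the parent actor of a 2D puzzle, wiring its child handles and puzzle nodes together at construction time.
; The construction script scans child actors, storing the BP_Handle with HandleNum 1 as left and any other as right.
; A second pass gives each BP_PuzzleNode its matching parent handle and a red (left) or blue (right) laser pointer spline mesh.
; The event graph holds no active logic.
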(event EventBeginPlay)

(event Collision|EventActorBeginOverlap
  (params (OtherActor :type Actor%20Object%20Reference)))

(event EventTick
  (params (DeltaSeconds :type Float%20%28single-precision%29)))

(fn ConstructionScript
  (bind _childactors (Actor|GetAllChildActors true))
  (for _array_element _childactors
    (bind _asbp_handle (Utilities|Casting|CastToBP_Handle _array_element))
    (if (== (Variables|/Game/Blueprints/2Dpuzzle/BP_Handle.BP_Handle_C|GetHandleNum _asbp_handle) 1)
      (Variables|Default|SetLeftHandleBP _asbp_handle)
      (else
        (Variables|Default|SetRightHandleBP _asbp_handle))))
  (for _array_element_2 _childactors
    (bind _asbp_puzzle_node (Utilities|Casting|CastToBP_PuzzleNode _array_element_2))
    (if (== (Variables|/Game/Blueprints/2Dpuzzle/BP_PuzzleNode.BP_PuzzleNode_C|GetHandleNum _asbp_puzzle_node) 1)
      (Variables|/Game/Blueprints/2Dpuzzle/BP_PuzzleNode.BP_PuzzleNode_C|SetParentHandle _asbp_puzzle_node (Variables|Default|GetLeftHandleBP))
      (Components|StaticMesh|SetStaticMesh (Variables|/Game/Blueprints/2Dpuzzle/BP_PuzzleNode.BP_PuzzleNode_C|GetSplineMesh _asbp_puzzle_node) "/Engine/LaserPointerMesh_RED.LaserPointerMesh_RED")
      (else
        (Variables|/Game/Blueprints/2Dpuzzle/BP_PuzzleNode.BP_PuzzleNode_C|SetParentHandle _asbp_puzzle_node (Variables|Default|GetRightHandleBP))
        (Components|StaticMesh|SetStaticMesh (Variables|/Game/Blueprints/2Dpuzzle/BP_PuzzleNode.BP_PuzzleNode_C|GetSplineMesh _asbp_puzzle_node) "/Engine/VREditor/LaserPointer/LaserPointerMesh_BLUE.LaserPointerMesh_BLUE")))))