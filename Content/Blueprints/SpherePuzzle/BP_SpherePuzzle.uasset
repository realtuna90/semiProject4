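; A motion-controller-grabbable sphere puzzle with green, red and yellow lines to complete.
; Pickup attaches it to the given component and fires StartPuzzle once, while Tick pins it to its construction location.
; Tick also hides unfinished lines when no color is active.
; It registers with SpherePuzzleManager on BeginPlay; the third Line event fires ClearPuzzle and activates RotatingMovement.
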(event Custom|Line
  (Variables|Default|SetClear (+ (Variables|Default|GetClear) 1))
  (if (== (Variables|Default|GetClear) 3)
    (Default|CallClearPuzzle)
    (Components|Activation|Activate (Variables|Default|GetRotatingMovement) false)))

(event EventDrop
  (Transformation|DetachFromActor "KeepWorld" "KeepWorld" "KeepWorld"))

(event EventBeginPlay
  (bind _returnvalue (Actor|GetActorOfClass "/Game/Blueprints/SpherePuzzle/SpherePuzzleManager.SpherePuzzleManager_C"))
  (Utilities|IsValid _returnvalue
    (:Is%20Valid
      (Variables|/Game/Blueprints/SpherePuzzle/SpherePuzzleManager.SpherePuzzleManager_C|SetPuzzle _returnvalue self))))

(event EventPickup
  (params (AttachTo :type Scene%20Component%20Object%20Reference) (MotionController :type BP%20Motion%20Controller%20Object%20Reference))
  (Physics|SetSimulatePhysics (Variables|Default|GetSphere) false)
  (Transformation|AttachComponentToComponent (VehicleSound|GetRootComponent) AttachTo "None" "KeepWorld" "KeepWorld" "KeepWorld" false)
  (Utilities|FlowControl|DoOnce false
    (:Completed
      (Default|CallStartPuzzle MotionController))))

(event EventTick
  (params (DeltaSeconds :type Float%20%28single-precision%29))
  (Utilities|FlowControl|Sequence
    (:then_0
      (Transformation|SetActorLocation (Variables|Default|GetInitialLocation) false false))
    (:then_1
      (if (Utilities|Text|TextIsEmpty (Variables|Default|GetNowColor))
        (Utilities|FlowControl|Sequence
          (:then_0
            (if (not (Variables|Default|GetGreenOver))
              (Rendering|SetVisibility (Variables|Default|GetLine_Green) false false)))
          (:then_1
            (if (not (Variables|Default|GetRedOver))
              (Rendering|SetVisibility (Variables|Default|GetLine_Red) false false)))
          (:then_2
            (if (not (Variables|Default|GetYellowOver))
              (Rendering|SetVisibility (Variables|Default|GetLine_Yellow) false false))))))))

(fn ConstructionScript
  (Variables|Default|SetInitialLocation (Transformation|GetActorLocation)))