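; BP_Handle is a grabbable VR handle in the 2D puzzle folder that rotates its mesh with the hand holding it.
; Pickup records starting mesh and controller angles, using Yaw to resolve Pitch, and fires HandleControlOn; Drop stops rotation and fires HandleControlOff.
; While held, Tick projects the hand's right vector onto the plane normal to the actor's right vector, applies the starting offset and sets mesh rotation from it.
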(event EventPickup
  (params (AttachTo :type Scene%20Component%20Object%20Reference) (MotionController :type BP%20Motion%20Controller%20Object%20Reference))
  (bind _returnvalue (Transformation|GetActorRightVector))
  (bind _returnvalue_2 (Math|Vector|MakeVector 0.0 0.0 0.0))
  (bind _staticmesh (Variables|Default|GetStaticMesh))
  (bind _handmesh (Variables|/Game/Blueprints/BP_MotionController.BP_MotionController_C|GetHandMesh MotionController))
  (bind _returnvalue_3 (Math|Vector|GetRightVector _handmesh))
  (bind _relativerotation (Variables|/Script/Engine.SceneComponent|GetRelativeRotation _staticmesh))
  (bind _returnvalue_4 (Math|Vector|ProjectVectorontoPlane _returnvalue_3 _returnvalue))
  (bind _returnvalue_5 (Math|Vector|Normalize _returnvalue_4))
  (bind _returnvalue_6 (Math|Rotator|FindLookatRotation _returnvalue_2 _returnvalue_5))
  (Default|CallHandleControlon)
  (Variables|Default|SetIsRotating true)
  (Utilities|FlowControl|Sequence
    (:then_0
      (if (== (.yaw _relativerotation) 0.0)
        (Variables|Default|SetInitialMeshRotation (- 1.8e+02 (.pitch _relativerotation)))
        (else
          (Variables|Default|SetInitialMeshRotation (.pitch _relativerotation)))))
    (:then_1
      (if (== (.yaw _returnvalue_6) 0.0)
        (Variables|Default|SetInitialControllerRotation (- 1.8e+02 (.pitch _returnvalue_6)))
        (else
          (Variables|Default|SetInitialControllerRotation (.pitch _returnvalue_6)))))))

(event EventTick
  (params (DeltaSeconds :type Float%20%28single-precision%29))
  (bind _returnvalue (Transformation|GetActorRightVector))
  (Utilities|FlowControl|Sequence
    (:then_0
      (if (Variables|Default|GetIsRotating)
        (Transformation|SetRelativeRotation (Variables|Default|GetStaticMesh) (Math|Rotator|FindLookatRotation (Math|Vector|MakeVector 0.0 0.0 0.0) (Math|Vector|RotateVectorAroundAxis (Math|Vector|Normalize (Math|Vector|ProjectVectorontoPlane (Math|Vector|GetRightVector (Variables|/Game/Blueprints/BP_MotionController.BP_MotionController_C|GetHandMesh (stale EventPickup MotionController))) _returnvalue)) (- (Variables|Default|GetInitialMeshRotation) (Variables|Default|GetInitialControllerRotation)) _returnvalue)) false false)))))

(event EventDrop
  (Default|CallHandleControlOff)
  (Variables|Default|SetIsRotating false))

(fn ConstructionScript)