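; BP_Button is a physical VR push button that triggers a blast when pressed and released.
; Each tick it follows the overlapping component's local Z travel, clamped to a maximum depth, and eases back when free.
; Release past half depth calls CallPressed, then activates BOOM's force component and damps the MotionControllerPawn's physics root for two seconds.
; A highlight mesh hides on touch; an impulse branch on the pawn is left unwired.
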(event OnComponentBeginOverlap(Button)
  (params (OverlappedComponent :type Primitive%20Component%20Object%20Reference) (OtherActor :type Actor%20Object%20Reference) (OtherComp :type Primitive%20Component%20Object%20Reference) (OtherBodyIndex :type Integer) (bFromSweep :type Boolean) (SweepResult :type Hit%20Result%20Structure%20%28by%20ref%29))
  (Utilities|IsValid (Variables|Default|GetoverlappedComponent)
    (:Is%20Not%20Valid
      (bind _output_get (Variables|Default|SetoverlappedComponent OtherComp))
      (Variables|Default|SetinitialOverlapLocation (Transformation|GetWorldLocation _output_get))
      (CallFunction|HighLightOff))))

(event OnComponentEndOverlap(Button)
  (params (OverlappedComponent :type Primitive%20Component%20Object%20Reference) (OtherActor :type Actor%20Object%20Reference) (OtherComp :type Primitive%20Component%20Object%20Reference) (OtherBodyIndex :type Integer))
  (bind _boom (Variables|Default|GetBOOM))
  (bind _forcecomponent (Variables|/Script/Engine.RadialForceActor|GetForceComponent _boom))
  (if (== OtherComp (Variables|Default|GetoverlappedComponent))
    (Variables|Default|SetoverlappedComponent 0)
    (if (> (Variables|Default|GetbuttonPressAmount) (* (Variables|Default|GetmaxButtonPressAmount) 0.5))
      (Default|CallPressed)
      (bind _asmotion_controller_pawn (Utilities|Casting|CastToMotionControllerPawn (Game|Player|GetPlayerPawn 0)))
      (Components|Activation|Activate _forcecomponent false)
      (Class|PrimitiveComponent|SetLinearDamping (Variables|/Game/Blueprints/MotionControllerPawn.MotionControllerPawn_C|GetPhysicsRoot _asmotion_controller_pawn) 2.0)
      (Utilities|FlowControl|Delay 2.0)
      (Components|Activation|Deactivate _forcecomponent)
      (Class|PrimitiveComponent|SetLinearDamping (Variables|/Game/Blueprints/MotionControllerPawn.MotionControllerPawn_C|GetPhysicsRoot _asmotion_controller_pawn) 0.0))))

(event EventHighLightOff
  (Rendering|SetVisibility (Variables|Default|GetHighLight) false false))

(event EventHighLighton
  (Rendering|SetVisibility (Variables|Default|GetHighLight) true false))

(event EventTick
  (params (DeltaSeconds :type Float%20%28single-precision%29))
  (bind _button (Variables|컴포넌트|GetButton))
  (bind _buttonroot (Variables|컴포넌트|GetButtonRoot))
  (Utilities|FlowControl|Sequence
    (:then_0
      (Utilities|IsValid (Variables|Default|GetoverlappedComponent)
        (:Is%20Valid
          (bind _output_get (Variables|Default|SetbuttonPressAmount (Math|Float|Clamp(Float) (.z (- (Math|Transform|InverseTransformLocation (Transformation|GetWorldTransform _buttonroot) (Variables|Default|GetinitialOverlapLocation)) (Math|Transform|InverseTransformLocation (Transformation|GetWorldTransform _buttonroot) (Transformation|GetWorldLocation (Variables|Default|GetoverlappedComponent))))) 0.0 (Variables|Default|GetmaxButtonPressAmount))))
          (Transformation|SetRelativeLocation _button (Math|Vector|MakeVector 0.0 0.0 (* _output_get -1.0)) false false))
        (:Is%20Not%20Valid
          (Transformation|SetRelativeLocation _button (Math|Interpolation|VInterpTo (Variables|/Script/Engine.SceneComponent|GetRelativeLocation (Variables|컴포넌트|GetButton)) "0, 0, 0" DeltaSeconds 0.0) false false))))))

(fn ConstructionScript)