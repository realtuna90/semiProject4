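; BP_FingerPrintDoor is a sliding door that registers with BP_AutoDoorManager and opens through a sensor-driven event.
; A timeline lerps the door mesh between closed and open positions and plays the sound.
; Tick holds a countdown that refreshes while the first stored sensor is overlapped.
; Closing reverses the timeline once the countdown expires and the ZoneTrigger's non-static-mesh actor count equals two, polling with zero-length Delays.
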(event Custom|DoorOpen_Event
  (params (Sensor :type BP%20Finger%20Print%20Object%20Reference))
  (Utilities|FlowControl|Sequence
    (:then_0
      (Utilities|FlowControl|DoOnce false
        (:Completed
          (Variables|Default|SetSensor Sensor))))
    (:then_1
      (Variables|Default|SetIsOpen true)
      (Variables|Default|SetopenTime 4.25)
      (bind _doorposition (Timeline|Timeline_0 Play)
        (:Update
          (Transformation|SetRelativeLocation (Variables|Default|GetSM_CConsoleSModuleB) (Math|Vector|Lerp(Vector) (Variables|DoorSetup|GetDoorClose) (Variables|DoorSetup|GetDoorOpen) _doorposition) false false) ; The new location is based on the vectors and triggered by the 'TimeLine' node
        )
        (:Finished
          (if (Variables|Default|GetIsOpen)
            (CallFunction|Close)))
        (:SoundTiming
          (Audio|PlaySoundatLocation "/Game/SciFiPopulate/Maps/DemoLevel/Sounds/Futuristic_door.Futuristic_door" (Transformation|GetActorLocation) "0, 0, 0" 0.1 1.5 0.0 0 0 0))))))

(event Custom|close
  (bind _zonetrigger (Variables|Default|GetZoneTrigger))
  (if (or (Variables|Default|GetIsOpen) (!= (- (Utilities|Array|Length (Collision|GetOverlappingActors _zonetrigger "/Script/Engine.Actor" :!class /Script/Engine.PrimitiveComponent)) (Utilities|Array|Length (Collision|GetOverlappingActors _zonetrigger "/Script/Engine.StaticMeshActor" :!class /Script/Engine.PrimitiveComponent))) 2)) :!label _label
    (Utilities|FlowControl|Delay 0.0)
    (goto _label)
    (else
      (bind _doorposition (Timeline|Timeline_0 Reverse)
        (:Update
          (Transformation|SetRelativeLocation (Variables|Default|GetSM_CConsoleSModuleB) (Math|Vector|Lerp(Vector) (Variables|DoorSetup|GetDoorClose) (Variables|DoorSetup|GetDoorOpen) _doorposition) false false) ; The new location is based on the vectors and triggered by the 'TimeLine' node
        )
        (:Finished
          (if (Variables|Default|GetIsOpen)
            (CallFunction|Close)))
        (:SoundTiming
          (Audio|PlaySoundatLocation "/Game/SciFiPopulate/Maps/DemoLevel/Sounds/Futuristic_door.Futuristic_door" (Transformation|GetActorLocation) "0, 0, 0" 0.1 1.5 0.0 0 0 0))))))

(event EventBeginPlay
  (bind _returnvalue (Actor|GetActorOfClass "/Game/Blueprints/AutoDoor/BP_AutoDoorManager.BP_AutoDoorManager_C"))
  (Utilities|Array|AddUnique (Variables|/Game/Blueprints/AutoDoor/BP_AutoDoorManager.BP_AutoDoorManager_C|GetDoors _returnvalue) self))

(event EventTick
  (params (DeltaSeconds :type Float%20%28single-precision%29))
  (if (Variables|Default|GetIsOpen)
    (if (Variables|/Game/Blueprints/AutoDoor/BP_FingerPrint.BP_FingerPrint_C|GetIs%20Overlap (stale Custom|DoorOpen_Event Sensor)) :!label _label
      (Variables|Default|SetopenTime 4.0)
      (Utilities|FlowControl|Delay 0.0)
      (goto _label)
      (elif (< (- (Variables|Default|GetopenTime) DeltaSeconds) 0.0)
        (Variables|Default|SetIsOpen false)
        (else
          (Variables|Default|SetopenTime (- (Variables|Default|GetopenTime) DeltaSeconds)))))))

(fn ConstructionScript)