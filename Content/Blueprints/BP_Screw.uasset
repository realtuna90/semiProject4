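; BP_Screw is a screw on a panel that can be pulled out, then picked up and dropped.
; Each PullOut event raises and spins the mesh a step, switching off the panel's screw highlight on the first pull.
; At the travel limit it enables physics, ignores one trace channel and notifies the panel actor.
; Pickup and Drop toggle physics and attachment only after extraction; its own child-actor highlight starts off.
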(event Custom|PullOut_Event
  (bind _screwcomponent (Variables|Default|GetScrewComponent))
  (bind _screwcomponent_2 (Variables|Default|GetScrewComponent))
  (bind _screwcomponent_3 (Variables|Default|GetScrewComponent))
  (if (< (Variables|Default|GetPullAmount) (Variables|Default|GetMaxAmount))
    (Utilities|FlowControl|Sequence
      (:then_0
        (Variables|Default|SetPullAmount (+ (Variables|Default|GetPullAmount) 0.1))
        (Transformation|SetRelativeLocation _screwcomponent_3 (Math|Vector|MakeVector 0.0 0.0 (+ (.z (Variables|/Script/Engine.SceneComponent|GetRelativeLocation _screwcomponent_3)) 0.1)) false false))
      (:then_1
        (Transformation|SetRelativeRotation _screwcomponent_2 (Math|Rotator|MakeRotator 0.0 0.0 (+ (.yaw (Variables|/Script/Engine.SceneComponent|GetRelativeRotation _screwcomponent_2)) 1.0)) false false))
      (:then_2
        (Utilities|FlowControl|DoOnce false
          (:Completed
            (Default|ScrewHighLightOff (Variables|Default|GetPanelActor))))))
    (else
      (Physics|SetSimulatePhysics _screwcomponent true)
      (Collision|SetCollisionResponsetoChannel _screwcomponent "ECC_GameTraceChannel2" "ECR_Ignore")
      (Variables|Default|SetPullOutOver true)
      (Default|ScrewOut (Variables|Default|GetPanelActor) self))))

(event EventPickup
  (params (AttachTo :type Scene%20Component%20Object%20Reference) (MotionController :type BP%20Motion%20Controller%20Object%20Reference))
  (bind _screwcomponent (Variables|Default|GetScrewComponent))
  (if (Variables|Default|GetPullOutOver)
    (Physics|SetSimulatePhysics _screwcomponent false)
    (Transformation|AttachComponentToComponent _screwcomponent AttachTo "None" "KeepWorld" "KeepWorld" "KeepWorld" false)))

(event EventDrop
  (if (Variables|Default|GetPullOutOver)
    (Physics|SetSimulatePhysics (Variables|Default|GetScrewComponent) true)
    (Transformation|DetachFromActor "KeepWorld" "KeepWorld" "KeepWorld")))

(event EventBeginPlay
  (Utilities|FlowControl|Sequence
    (:then_0
      (bind _asbp_high_light (Utilities|Casting|CastToBP_HighLight (Variables|/Script/Engine.ChildActorComponent|GetChildActor (Variables|Default|GetBP_HighLight))))
      (bind _output_get (Variables|Default|SetHighLight _asbp_high_light))
      (Default|HighLighton _output_get false))
    (:then_1
      (EventDispatchers|BindEventtoPullOut (delegate Custom|PullOut_Event)))))

(fn ConstructionScript)