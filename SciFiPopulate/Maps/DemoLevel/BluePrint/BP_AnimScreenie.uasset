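; BP_AnimScreenie is an animated screen prop with a point light, driven by three capsule overlap volumes.
; Entering Capsule plays the first screen animation; leaving restarts it at zero play rate to hide it.
; Leaving Capsule1 plays the second animation, and all three animation triggers share one sound.
; Capsule2 plays and reverses a timeline that fades the light's intensity in and out.
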(event OnComponentBeginOverlap(Capsule2)
  (params (OverlappedComponent :type Primitive%20Component%20Object%20Reference) (OtherActor :type Actor%20Object%20Reference) (OtherComp :type Primitive%20Component%20Object%20Reference) (OtherBodyIndex :type Integer) (bFromSweep :type Boolean) (SweepResult :type Hit%20Result%20Structure%20%28by%20ref%29))
  ;[1 1 1] The PointLight will be switched ON if the player begins to collide with the 'Capsule2' collision. The intensity is set to '0' by default and on 'BeginOverlap' the intensity of the light will be multiplicated by the float (3500 here, it need to be tested in RealTime when created). In the 'TimeLine' node the soft bezier curve of 1s ensures that the light will be switched ON/OFF in a soft manner (ie: progressive way nonlinear)
  (bind _lightint (Timeline|Timeline_0 Play)
    (:Update
      (Rendering|Components|Light|SetIntensity (Variables|Default|GetPointLight) (* _lightint 3.5e+03)))))

(event OnComponentEndOverlap(Capsule2)
  (params (OverlappedComponent :type Primitive%20Component%20Object%20Reference) (OtherActor :type Actor%20Object%20Reference) (OtherComp :type Primitive%20Component%20Object%20Reference) (OtherBodyIndex :type Integer))
  ;[1 1 1] The PointLight will be switched OFF if the player ends to collide with the 'Capsule2' collision: reverse action
  ;[1 1 1] The PointLight will be switched ON if the player begins to collide with the 'Capsule2' collision. The intensity is set to '0' by default and on 'BeginOverlap' the intensity of the light will be multiplicated by the float (3500 here, it need to be tested in RealTime when created). In the 'TimeLine' node the soft bezier curve of 1s ensures that the light will be switched ON/OFF in a soft manner (ie: progressive way nonlinear)
  (bind _lightint (Timeline|Timeline_0 Reverse)
    (:Update
      (Rendering|Components|Light|SetIntensity (Variables|Default|GetPointLight) (* _lightint 3.5e+03)))))

(event OnComponentEndOverlap(Capsule)
  (params (OverlappedComponent :type Primitive%20Component%20Object%20Reference) (OtherActor :type Actor%20Object%20Reference) (OtherComp :type Primitive%20Component%20Object%20Reference) (OtherBodyIndex :type Integer))
  ;[1 1 1] Since the play rate is set to '0', the skeletal mesh 'SK_ScreenieAnim1' will disappear if the player ends to collide with the 'Capsule' collision. Thus we can see clearly the 'SK_ScreenieAnim2' animation
  (Components|Animation|PlayAnimation (Variables|Default|GetSK_ScreenieAnim1) "/Game/SciFiPopulate/SkeletalMeshes/SK_ScreenieAnim1_Anim.SK_ScreenieAnim1_Anim" false)
  (Components|Timeline|SetPlayRate (Variables|Default|GetSK_ScreenieAnim1) 0.0)
  ;[1 1 1] A sound is played when each animation of the screenie is played, no matter the animation (1 or 2) = same sound
  (Audio|PlaySoundatLocation "/Engine/EditorSounds/Notifications/CompileSuccess.CompileSuccess" "0, 0, 0" "0, 0, 0" 0.4 1.2))

(event OnComponentEndOverlap(Capsule1)
  (params (OverlappedComponent :type Primitive%20Component%20Object%20Reference) (OtherActor :type Actor%20Object%20Reference) (OtherComp :type Primitive%20Component%20Object%20Reference) (OtherBodyIndex :type Integer))
  ;[1 1 1] The animation 'SK_ScreenieAnim2_Anim' will be played by the 'SK_ScreenieAnim2' if the player ends to collide with the 'Capsule1' collision
  (Components|Animation|PlayAnimation (Variables|Default|GetSK_ScreenieAnim2) "/Game/SciFiPopulate/SkeletalMeshes/SK_ScreenieAnim2_Anim.SK_ScreenieAnim2_Anim" false)
  ;[1 1 1] A sound is played when each animation of the screenie is played, no matter the animation (1 or 2) = same sound
  (Audio|PlaySoundatLocation "/Engine/EditorSounds/Notifications/CompileSuccess.CompileSuccess" "0, 0, 0" "0, 0, 0" 0.4 1.2))

(event OnComponentBeginOverlap(Capsule)
  (params (OverlappedComponent :type Primitive%20Component%20Object%20Reference) (OtherActor :type Actor%20Object%20Reference) (OtherComp :type Primitive%20Component%20Object%20Reference) (OtherBodyIndex :type Integer) (bFromSweep :type Boolean) (SweepResult :type Hit%20Result%20Structure%20%28by%20ref%29))
  ;[1 1 1] The animation 'SK_ScreenieAnim1_Anim' will be played by the 'SK_ScreenieAnim1' if the player begins to collide with the 'Capsule' collision
  (Components|Animation|PlayAnimation (Variables|Default|GetSK_ScreenieAnim1) "/Game/SciFiPopulate/SkeletalMeshes/SK_ScreenieAnim1_Anim.SK_ScreenieAnim1_Anim" false)
  ;[1 1 1] A sound is played when each animation of the screenie is played, no matter the animation (1 or 2) = same sound
  (Audio|PlaySoundatLocation "/Engine/EditorSounds/Notifications/CompileSuccess.CompileSuccess" "0, 0, 0" "0, 0, 0" 0.4 1.2))

(fn ConstructionScript)