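; Pipe prop for the space walk that can be picked up, dropped and made to smoke.
; Unless Throwaway is set, Tick follows IsSmoking through two DoOnce gates that reset each other, so each change acts once.
; Smoking turns on Smoke1 and disables mesh collision; stopping reverses both.
; Pickup disables physics and attaches the mesh to the given component, while Drop re-enables physics and detaches.
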(event EventPickup
  (params (AttachTo :type Scene%20Component%20Object%20Reference) (MotionController :type BP%20Motion%20Controller%20Object%20Reference))
  (bind _staticmesh (Variables|Default|GetStaticMesh))
  (Physics|SetSimulatePhysics _staticmesh false)
  (Transformation|AttachComponentToComponent _staticmesh AttachTo "None" "KeepWorld" "KeepWorld" "KeepWorld" false))

(event EventTick
  (params (DeltaSeconds :type Float%20%28single-precision%29))
  (bind _staticmesh (Variables|Default|GetStaticMesh))
  (if (not (Variables|Default|GetThrowaway?))
    (if (Variables|Default|GetIsSmoking)
      (Utilities|FlowControl|DoOnce false :!label _label
        (:Completed
          (Components|Activation|Activate (Variables|Default|GetSmoke1) false)
          (Collision|SetCollisionEnabled _staticmesh "NoCollision")
          (goto _label_2 Reset)))
      (else
        (Utilities|FlowControl|DoOnce false :!label _label_2
          (:Completed
            (Components|Activation|Deactivate (Variables|Default|GetSmoke1))
            (Collision|SetCollisionEnabled _staticmesh "QueryAndPhysics")
            (goto _label Reset)))))))

(event EventDrop
  (Physics|SetSimulatePhysics (Variables|Default|GetStaticMesh) true)
  (Transformation|DetachFromActor "KeepWorld" "KeepWorld" "KeepWorld"))

(fn ConstructionScript)