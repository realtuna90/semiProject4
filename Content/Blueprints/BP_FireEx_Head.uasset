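; BP_FireEx_Head is an equippable piece, by its name a fire extinguisher head, that can be held and returned to its parent component.
; It caches that parent component on BeginPlay.
; Equip attaches it to the given component's right-hand socket, keeping its world transform.
; Drop detaches it and snaps it back onto the cached parent; both events disable mesh physics and update the equipped flag.
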(event EventEquip
  (params (EquipTo :type Scene%20Component%20Object%20Reference))
  (Physics|SetSimulatePhysics (Variables|Default|GetStaticMeshComponent) false)
  (Transformation|AttachComponentToComponent (VehicleSound|GetRootComponent) EquipTo "SocketRightHand" "KeepWorld" "KeepWorld" "KeepWorld" false)
  (Variables|Default|SetisEquipped true))

(event EventDrop
  (Physics|SetSimulatePhysics (Variables|Default|GetStaticMeshComponent) false)
  (Transformation|DetachFromActor "KeepWorld" "KeepWorld" "KeepWorld")
  (Variables|Default|SetisEquipped false)
  (Transformation|AttachComponentToComponent (Variables|Default|Getparent) "None" "SnapToTarget" "SnapToTarget" "KeepRelative" true))

(event EventBeginPlay
  (Variables|Default|Setparent (Class|Actor|GetParentComponent)))

(fn ConstructionScript)