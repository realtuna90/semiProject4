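; BP_Explode triggers an explosion in the SpaceWalk content when the BP_Valve actor fires its Explode event.
; On BeginPlay it finds the valve by class and binds to that dispatcher.
; The explosion enables physics simulation on components overlapping its Box, skipping the motion controller pawn and controllers.
; It then pulses the BOOM force component briefly to push the loosened objects.
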(event Custom|Explosion
  (bind _boom (Variables|Default|GetBOOM))
  (bind _forcecomponent (Variables|/Script/Engine.RadialForceActor|GetForceComponent _boom))
  (for _array_element (Class|PrimitiveComponent|GetOverlappingComponents (Variables|Default|GetBox))
    (Utilities|Casting|CastToMotionControllerPawn (Components|GetOwner _array_element)
      (:CastFailed
        (Utilities|Casting|CastToBP_MotionController (Components|GetOwner _array_element)
          (:CastFailed
            (Physics|SetSimulatePhysics _array_element true))))))
  (Components|Activation|Activate _forcecomponent false)
  (Utilities|FlowControl|Delay 0.2)
  (Components|Activation|Deactivate _forcecomponent))

(event EventBeginPlay
  (bind _returnvalue (Actor|GetActorOfClass "/Game/Blueprints/SpaceWalk/BP_Valve.BP_Valve_C"))
  (bind _output_get (Variables|Default|SetValve _returnvalue))
  (EventDispatchers|BindEventtoExplode _output_get (delegate Custom|Explosion)))

(fn ConstructionScript)