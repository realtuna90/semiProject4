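; An actor component that shows its owner as a point of interest on the VR player's arm minimap during a given stage and phase.
; It listens to the VRGameMode phase change event from BeginPlay.
; On a match, after a short delay, it adds the owner to the minimap on the pawn's left controller arm widget and stores the returned widget.
; Otherwise, it removes that widget.
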(event Custom|OnChangePhase
  (params (Stage :type LevelEnum%20Enum :default "NewEnumerator4") (Phase :type Integer))
  (if (and (Utilities|Enum|Equal(Enum) Stage (Variables|Default|GetStage)) (== (Variables|Default|GetPhase) Phase))
    (Utilities|FlowControl|Delay 0.2)
    (bind _asmotion_controller_pawn (Utilities|Casting|CastToMotionControllerPawn (Game|Player|GetPlayerPawn 0)))
    (bind _widget (Default|AddPOI (Variables|/Game/Blueprints/Arm_Widget.Arm_Widget_C|GetMinimap_Widget2 (Variables|/Game/Blueprints/BP_MotionController.BP_MotionController_C|GetArmWidget (Variables|/Game/Blueprints/MotionControllerPawn.MotionControllerPawn_C|GetLeftController _asmotion_controller_pawn))) (Components|GetOwner)))
    (Variables|Default|SetWidget _widget)
    (else
      (Utilities|IsValid (Variables|Default|GetWidget)
        (:Is%20Valid
          (Widget|RemovefromParent (Variables|Default|GetWidget)))))))

(event EventBeginPlay
  (bind _asvrgame_mode (Utilities|Casting|CastToVRGameMode (Game|GetGameMode)))
  (EventDispatchers|BindEventtoOnChangePhase _asvrgame_mode (delegate Custom|OnChangePhase)))