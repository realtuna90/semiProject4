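; BP_HighLight is an arrow marker that starts hidden and can be switched on and off as a highlight.
; HighLightOn shows ArrowMesh with an accent or basic material, and HighLightOff hides it.
; Both call the HighLightControl dispatcher, bound at BeginPlay to play or stop a timeline.
; The timeline animates the arrow vertically by adding MovingZ as a relative delta each update, so offsets accumulate rather than set an absolute height.
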(event Custom|ControlEvent
  (params (Active :type Boolean))
  (if Active
    (bind _movingz (Timeline|타임라인_0 Play)
      (:Update
        (Transformation|AddRelativeLocation (Variables|Default|GetArrowMesh) (Math|Vector|MakeVector 0.0 0.0 _movingz) false false)))
    (else
      (Timeline|타임라인_0 Stop))))

(event EventBeginPlay
  (Rendering|SetVisibility (Variables|Default|GetArrowMesh) false false)
  (Variables|Default|SetownerActor (Components|GetOwner (Variables|Default|GetArrowMesh)))
  (EventDispatchers|BindEventtoHighLightControl (delegate Custom|ControlEvent)))

(fn ConstructionScript)

(fn HighLighton
  (params (Accent :type Boolean))
  (bind _arrowmesh (Variables|Default|GetArrowMesh))
  (Rendering|SetVisibility (Variables|Default|GetArrowMesh) true false)
  (if Accent
    (Rendering|Material|SetMaterial _arrowmesh 0 (Variables|Default|GetmaterialAccent))
    (else
      (Rendering|Material|SetMaterial _arrowmesh 0 (Variables|Default|GetmatrialBasic))))
  (Default|CallHighLightControl true))

(fn HighLightOff
  (Rendering|SetVisibility (Variables|Default|GetArrowMesh) false false)
  (Default|CallHighLightControl false))