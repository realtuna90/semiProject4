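; VR swing lever that a motion controller grabs and pulls to trigger a lever input.
; While held, Tick converts the grab sphere position into actor-local space and uses atan2 to set the lever's clamped pitch.
; On drop, a timeline lerps the lever back to its initial rotation, blocking dragging and triggering until finished.
; Lever overlap with FinalPullBox at other times calls the lever input.
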(event OnComponentBeginOverlap(FinalPullBox)
  (params (OverlappedComponent :type Primitive%20Component%20Object%20Reference) (OtherActor :type Actor%20Object%20Reference) (OtherComp :type Primitive%20Component%20Object%20Reference) (OtherBodyIndex :type Integer) (bFromSweep :type Boolean) (SweepResult :type Hit%20Result%20Structure%20%28by%20ref%29))
  (if (== OtherComp (Variables|Default|GetLever))
    (if (not (Variables|Default|GetResettingRotation))
      (Default|CallLeverInput))))

(event EventTick
  (params (DeltaSeconds :type Float%20%28single-precision%29))
  (bind _returnvalue (Transformation|GetActorTransform))
  (bind _leverrotate (Variables|Default|GetLeverRotate))
  (bind _bp_motioncontroller (Variables|Default|GetBP_MotionController))
  (bind _grabsphere (Variables|/Game/Blueprints/BP_MotionController.BP_MotionController_C|GetGrabSphere _bp_motioncontroller))
  (bind _relativelocation (Variables|/Script/Engine.SceneComponent|GetRelativeLocation _leverrotate))
  (bind _returnvalue_2 (Transformation|GetWorldLocation _grabsphere))
  (bind _returnvalue_3 (Math|Transform|InverseTransformLocation _returnvalue _returnvalue_2))
  (bind _returnvalue_4 (- _returnvalue_3 _relativelocation))
  (Utilities|IsValid (Variables|Default|GetBP_MotionController)
    (:Is%20Valid
      (if (Variables|Default|GetIsdrag)
        (if (not (Variables|Default|GetResettingRotation))
          (Transformation|SetRelativeRotation (Variables|Default|GetLeverRotate) (Math|Rotator|MakeRotator 0.0 (Math|Float|Clamp(Float) (Class|KismetMathLibrary|DegAtan2 (.z _returnvalue_4) (.x _returnvalue_4)) (Variables|Default|GetMinPitch) (Variables|Default|GetMaxPitch)) 0.0) false false))))))

(event EventPickup
  (params (AttachTo :type Scene%20Component%20Object%20Reference) (MotionController :type BP%20Motion%20Controller%20Object%20Reference))
  (Variables|Default|SetBP_MotionController MotionController)
  (Variables|Default|SetIsdrag true))

(event EventDrop
  (Variables|Default|SetIsdrag false)
  (Variables|Default|SetResettingRotation true)
  (Variables|Default|SetInterpLeverRotation (Variables|/Script/Engine.SceneComponent|GetRelativeRotation (Variables|Default|GetLeverRotate)))
  (bind _새_트랙_0 (Timeline|타임라인_0 PlayFromStart)
    (:Update
      (Transformation|SetRelativeRotation (Variables|Default|GetLeverRotate) (Math|Rotator|Lerp(Rotator) (Variables|Default|GetInterpLeverRotation) (Variables|Default|GetInitialLeverRotation) _새_트랙_0) false false))
    (:Finished
      (Variables|Default|SetResettingRotation false))))

(fn ConstructionScript)