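; BP_Biotank is a bio tank with destructible glass whose breakage sets off the alarm bulb and clears the gas room.
; The glass fracture event fires once, turns on BP_AlarmBulb and deactivates the local fog in BP_GasRoom, finding both through GetActorOfClass.
; After a short delay, it disables the gas room's box collision and removes the tank's point-of-interest marker and widget.
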(event OnComponentFracture(SM_bio_tank_02_SM_bio_tank_glass_DM)
  (params (HitPoint :type Vector%20%28by%20ref%29 :default "0, 0, 0") (HitDirection :type Vector%20%28by%20ref%29 :default "0, 0, 0"))
  (bind _pointofinterest_component (Variables|Default|GetPointOfInterest_Component))
  (Utilities|FlowControl|DoOnce false
    (:Completed
      (Utilities|FlowControl|Sequence
        (:then_0
          (bind _returnvalue (Actor|GetActorOfClass "/Game/Blueprints/GasEvent/BP_AlarmBulb.BP_AlarmBulb_C"))
          (Default|Bulbon _returnvalue))
        (:then_1
          (bind _returnvalue_2 (Actor|GetActorOfClass "/Game/Blueprints/GasEvent/BP_GasRoom.BP_GasRoom_C"))
          (Components|Activation|Deactivate (Variables|/Game/Blueprints/GasEvent/BP_GasRoom.BP_GasRoom_C|GetP_LocalFog _returnvalue_2))
          (Utilities|FlowControl|Delay 4.0)
          (Collision|SetCollisionEnabled (Variables|/Game/Blueprints/GasEvent/BP_GasRoom.BP_GasRoom_C|GetBox _returnvalue_2) "NoCollision")
          (Components|Activation|Deactivate _pointofinterest_component)
          (Widget|RemovefromParent (Variables|/Game/Blueprints/PointOfInterest_Component.PointOfInterest_Component_C|GetWidget _pointofinterest_component)))))))

(fn ConstructionScript)