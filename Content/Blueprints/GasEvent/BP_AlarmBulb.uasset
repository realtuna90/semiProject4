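; BP_AlarmBulb is a rotating alarm light for the gas event, built from two spotlights and a RotatingMovement component.
; BeginPlay stops the rotation and hides both lights.
; BulbOn starts the spin and shows the lights, guarded by a DoOnce that is never reset.
; A delayed switch-off back to the idle state exists but is unconnected, so the alarm stays on once triggered.
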(event Custom|BulbOn
  (Utilities|FlowControl|DoOnce false
    (:Completed
      (Components|Activation|Activate (Variables|Default|GetRotatingMovement) false)
      (Rendering|SetVisibility (Variables|Default|GetSpotLight) true false)
      (Rendering|SetVisibility (Variables|Default|GetSpotLight1) true false))))

(event EventBeginPlay
  (Components|Activation|Deactivate (Variables|Default|GetRotatingMovement))
  (Rendering|SetVisibility (Variables|Default|GetSpotLight) false false)
  (Rendering|SetVisibility (Variables|Default|GetSpotLight1) false false))

(fn ConstructionScript)