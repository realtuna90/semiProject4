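; BP_DriverGun is an equippable tool that pulls out BP_Screw actors with a visible beam.
; While equipped and in use, it line-traces forward every Tick, then binds to and fires the hit screw's PullOut dispatcher.
; The bound Screw event snaps the SplineMesh beam to the impact point and spawns sparks.
; Otherwise the beam extends to full trace range, and it hides when the equipped gun is idle.
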(event Custom|Screw
  (bind _traceend (Variables|Default|GetTraceEnd))
  (bind _output_get (Variables|Default|SetonHit (.bBlockingHit (Collision|BreakHitResult (stale EventTick _outhit)))))
  (Transformation|SetWorldLocation _traceend (.Location (Collision|BreakHitResult (stale EventTick _outhit))) false false)
  (SplineMesh|SetEndPosition (Variables|Default|GetSplineMesh) (Variables|/Script/Engine.SceneComponent|GetRelativeLocation _traceend) _output_get)
  (Effects|SpawnEmitteratLocation "/Game/StarterContent/Particles/P_Sparks.P_Sparks" (.Location (Collision|BreakHitResult (stale EventTick _outhit))) "0, 0, 0" "0.100000,0.100000,0.100000"))

(event EventTick
  (params (DeltaSeconds :type Float%20%28single-precision%29))
  (bind _tracepoint (Variables|Default|GetTracePoint))
  (bind _tracepoint_2 (Variables|Default|GetTracePoint))
  (bind _splinemesh (Variables|Default|GetSplineMesh))
  (bind _returnvalue (Transformation|GetWorldLocation _tracepoint))
  (bind _relativelocation (Variables|/Script/Engine.SceneComponent|GetRelativeLocation _tracepoint_2))
  (if (Variables|Default|GetisEquipped)
    (if (Variables|Default|GetisUse)
      (Utilities|FlowControl|Sequence
        (:then_0
          (Variables|Default|SetonHit false)
          (bind _outhit (Collision|LineTraceByChannel _returnvalue (+ _returnvalue (* (Math|Vector|GetForwardVector (Transformation|GetWorldRotation _tracepoint)) 1e+03)) "TraceTypeQuery3" true 0 "ForOneFrame"))
          (bind _asbp_screw (Utilities|Casting|CastToBP_Screw (.HitActor (Collision|BreakHitResult _outhit))))
          (EventDispatchers|BindEventtoPullOut _asbp_screw (delegate Custom|Screw))
          (Default|CallPullOut _asbp_screw))
        (:then_1
          (if (Math|Boolean|Equal(Boolean) (Variables|Default|GetonHit) false)
            (SplineMesh|SetStartandEnd _splinemesh _relativelocation "0, 0, 0" (+ _relativelocation (* (Math|Vector|GetForwardVector (Variables|/Script/Engine.SceneComponent|GetRelativeRotation _tracepoint_2)) 1e+03)) "0, 0, 0" true :!class /Script/Engine.SplineMeshComponent)
            (Rendering|SetVisibility _splinemesh true false))))
      (else
        (Rendering|SetVisibility (Variables|Default|GetSplineMesh) false false)))))

(fn ConstructionScript
  (Variables|Default|SetHighLightMesh 0))