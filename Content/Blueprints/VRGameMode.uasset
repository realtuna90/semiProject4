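; VR game mode that runs game start, stage progression, level streaming and game over.
; Unloading the "cinematice" streamed level starts the game, resetting oxygen and advancing to Stage 0, while Tick drains oxygen.
; Depleted oxygen, or toxic and burn callbacks from the motion controller pawn, trigger game over, which streams the cinematic back in after a delay.
; Dispatchers broadcast start, game over, stage, level-load and oxygen changes.
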(event Custom|GameOver
  ;[1 1 1] 게임오버
  (Variables|Default|SetGameOver? true)
  (Default|CallOnGameOver)
  (Development|PrintString "GameOver" true true "(R=0.000000,G=0.660000,B=1.000000,A=1.000000)" 1e+01)
  (Utilities|FlowControl|Delay 3.0)
  (CallFunction|LoadLevel "cinematice" (Variables|Default|GetCurLoadLevelName)))

(event Custom|ToxicControl
  (params (damageAmount :type Integer))
  (if (== damageAmount 100)
    (CallFunction|GameOver)))

(event Custom|BurnControl
  (params (RemainHP :type Integer))
  (if (== RemainHP 0)
    (CallFunction|GameOver)))

(event Custom|StageChange
  (params (curlevel :type LevelEnum%20Enum :default "NewEnumerator0"))
  ;[1 1 1] 스테이지 전환
  (switch Utilities|FlowControl|Switch|SwitchonLevelEnum curlevel
    (:NewEnumerator4
      (bind _output_get (Variables|Default|Setlevel "NewEnumerator3"))
      (Default|CallOnChangeStage _output_get))
    (:NewEnumerator3
      (bind _output_get_2 (Variables|Default|Setlevel "NewEnumerator0"))
      (Default|CallOnChangeStage _output_get_2))
    (:NewEnumerator0
      (bind _output_get_3 (Variables|Default|Setlevel "NewEnumerator1"))
      (Default|CallOnChangeStage _output_get_3))
    (:NewEnumerator1
      (bind _output_get_4 (Variables|Default|Setlevel "NewEnumerator2"))
      (Default|CallOnChangeStage _output_get_4))
    (:NewEnumerator2
      (bind _output_get_5 (Variables|Default|Setlevel "NewEnumerator5"))
      (Default|CallOnChangeStage _output_get_5))))

(event Custom|GameStart
  ;[1 1 1] 게임 시작
  (Variables|Default|SetStart true)
  (Default|CallOnGameStart)
  (Development|PrintString "GameStart!!!" true true "(R=0.000000,G=0.660000,B=1.000000,A=1.000000)" 1e+01))

(event Custom|StartEvent
  (Variables|Default|SetOxygen 1.2e+03)
  (Variables|Default|SetOxygenControl 1.0)
  (CallFunction|StageChange "NewEnumerator4"))

(event Custom|OnLevelUnloaded_Event_0
  (CallFunction|GameStart))

(event Custom|LoadLevel
  (params (LoadLevel :type Name) (UnloadLevel :type Name))
  (if (Variables|Default|GetGameOver?)
    (Default|CallOnLevelLoad)
    (Game|LoadStreamLevel(byName) LoadLevel true)
    (Game|UnloadStreamLevel(byName) UnloadLevel false)
    (Variables|Default|SetCurLoadLevelName LoadLevel)
    (Variables|Default|SetGameOver? false)
    (else
      (Default|CallOnLevelLoad)
      (Game|LoadStreamLevel(byName) LoadLevel true)
      (Game|UnloadStreamLevel(byName) UnloadLevel false)
      (Variables|Default|SetCurLoadLevelName LoadLevel))))

(event Custom|GameOver_Event
  (Variables|Default|SetStart false)
  (Variables|Default|Setlevel "NewEnumerator4"))

(event EventBeginPlay
  (bind _returnvalue (Class|GameplayStatics|GetStreamingLevel "cinematice"))
  (Utilities|FlowControl|Sequence
    (:then_0
      (bind _asmotion_controller_pawn (Utilities|Casting|CastToMotionControllerPawn (Game|Player|GetPlayerPawn 0)))
      (EventDispatchers|BindEventtoToxicCallback _asmotion_controller_pawn (delegate Custom|ToxicControl)))
    (:then_1
      (EventDispatchers|BindEventtoBurnCallback _asmotion_controller_pawn (delegate Custom|BurnControl)))
    (:then_2
      (EventDispatchers|BindEventtoOnGameStart (delegate Custom|StartEvent)))
    (:then_3
      (Utilities|IsValid _returnvalue
        (:Is%20Valid
          (EventDispatchers|AssignOnLevelUnloaded _returnvalue (delegate Custom|OnLevelUnloaded_Event_0)))))
    (:then_4
      (EventDispatchers|BindEventtoOnGameOver (delegate Custom|GameOver_Event)))))

(event EventTick
  (params (DeltaSeconds :type Float%20%28single-precision%29))
  ;[1 1 1] 시간 체크
  (if (Variables|Default|GetStart)
    (if (> (Variables|Default|GetOxygen) 0.0)
      (bind _output_get (Variables|Default|SetOxygen (- (Variables|Default|GetOxygen) (* DeltaSeconds (Variables|Default|GetOxygenControl)))))
      (Default|CallOnDecreaseOxygen)
      (if (< _output_get 0.0)
        (Variables|Default|SetOxygen 0.0)
        (CallFunction|GameOver)))))

(fn ConstructionScript)