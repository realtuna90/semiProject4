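; BP_SpherePuzzle is a sphere puzzle actor that a motion controller can grab and that signals when the puzzle starts.
; Pickup disables the sphere's physics, attaches the root to the grabbing component and fires StartPuzzle with the controller on first grab only.
; Drop detaches it in world space.
; Tick resets the location captured at construction every frame, so the held sphere stays in place while its rotation remains free.
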(event EventDrop
  (Transformation|DetachFromActor "KeepWorld" "KeepWorld" "KeepWorld"))

(event EventPickup
  (params (AttachTo :type Scene%20Component%20Object%20Reference) (MotionController :type BP%20Motion%20Controller%20Object%20Reference))
  (Physics|SetSimulatePhysics (Variables|Default|GetSphere) false)
  (Transformation|AttachComponentToComponent (VehicleSound|GetRootComponent) AttachTo "None" "KeepWorld" "KeepWorld" "KeepWorld" false)
  (Utilities|FlowControl|DoOnce false
    (:Completed
      (Default|CallStartPuzzle MotionController))))

(event EventBeginPlay)

(event EventTick
  (params (DeltaSeconds :type Float%20%28single-precision%29))
  (Utilities|FlowControl|Sequence
    (:then_0
      (Transformation|SetActorLocation (Variables|Default|GetInitialLocation) false false))))

(fn ConstructionScript
  (Variables|Default|SetInitialLocation (Transformation|GetActorLocation)))