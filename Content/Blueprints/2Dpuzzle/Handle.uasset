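; A VR handle Blueprint in the 2D puzzle folder that turns its static mesh with the motion controller holding it.
; Pickup and Drop toggle rotation, and while held Tick projects the hand mesh's right vector onto the plane normal to the actor's right vector.
; The projected direction directly sets the mesh's relative rotation; the initial rotations saved on pickup are not used to offset it.
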(event EventPickup
  (params (AttachTo :type Scene%20Component%20Object%20Reference) (MotionController :type BP%20Motion%20Controller%20Object%20Reference))
  (bind _staticmesh (Variables|Default|GetStaticMesh))
  (Variables|Default|SetIsRotating true)
  (Variables|컴포넌트|SetInitialRotationHandle (Variables|/Script/Engine.SceneComponent|GetRelativeRotation _staticmesh))
  (Variables|Default|SetInitialRotatorController (Math|Rotator|FindLookatRotation (Math|Vector|MakeVector 0.0 0.0 0.0) (Math|Vector|Normalize (Math|Vector|ProjectVectorontoPlane (Math|Vector|RotateVector (Math|Vector|GetRightVector (Variables|/Game/Blueprints/BP_MotionController.BP_MotionController_C|GetHandMesh MotionController)) "0, 0, 0") (Transformation|GetActorRightVector)))))
  (Variables|Default|Setinitiallocation (Math|Vector|GetForwardVector _staticmesh)))

(event EventTick
  (params (DeltaSeconds :type Float%20%28single-precision%29))
  (if (Variables|Default|GetIsRotating)
    (Transformation|SetRelativeRotation (Variables|Default|GetStaticMesh) (Math|Rotator|FindLookatRotation (Math|Vector|MakeVector 0.0 0.0 0.0) (Math|Vector|Normalize (Math|Vector|ProjectVectorontoPlane (Math|Vector|RotateVector (Math|Vector|GetRightVector (Variables|/Game/Blueprints/BP_MotionController.BP_MotionController_C|GetHandMesh (stale EventPickup MotionController))) "0, 0, 0") (Transformation|GetActorRightVector)))) false false)))

(event EventDrop
  (Variables|Default|SetIsRotating false))

(fn ConstructionScript)