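; BP_Fire is a growing, extinguishable fire hazard that registers with BP_FireManager and damages the MotionControllerPawn.
; Tick enlarges it through Delay-throttled scaling; past a size threshold it spawns one child fire at a random position, flagged against further spreading.
; Sphere overlap enables periodic, escalating player damage.
; KillFire events shrink it until, below a minimum scale, it swaps flames for brief smoke, removes its PointOfInterest component and calls Extinguish.
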(event OnComponentBeginOverlap(Sphere)
  (params (OverlappedComponent :type Primitive%20Component%20Object%20Reference) (OtherActor :type Actor%20Object%20Reference) (OtherComp :type Primitive%20Component%20Object%20Reference) (OtherBodyIndex :type Integer) (bFromSweep :type Boolean) (SweepResult :type Hit%20Result%20Structure%20%28by%20ref%29))
  (Utilities|Casting|CastToMotionControllerPawn OtherActor)
  (Variables|Default|SetOnBurn true))

(event OnComponentEndOverlap(Sphere)
  (params (OverlappedComponent :type Primitive%20Component%20Object%20Reference) (OtherActor :type Actor%20Object%20Reference) (OtherComp :type Primitive%20Component%20Object%20Reference) (OtherBodyIndex :type Integer))
  (Utilities|Casting|CastToMotionControllerPawn OtherActor)
  (Variables|Default|SetOnBurn false))

(event Custom|KillFire_Event
  (bind _output_get (Variables|Default|SetFireScale (- (Variables|Default|GetFireScale) (Variables|Default|GetKillAmount))))
  (Transformation|SetWorldScale3D (Variables|Default|GetScene) (Math|Vector|MakeVector _output_get _output_get _output_get)))

(event EventTick
  (params (DeltaSeconds :type Float%20%28single-precision%29))
  (bind _scene (Variables|Default|GetScene))
  (bind _plusscaleamount (Variables|Default|GetplusScaleAmount))
  (bind _returnvalue (Transformation|GetWorldScale _scene))
  (bind _returnvalue_2 (+ (.y _returnvalue) _plusscaleamount))
  (if (< (Variables|Default|GetFireScale) 0.4)
    (Utilities|FlowControl|DoOnce false
      (:Completed
        (Components|Activation|Deactivate (Variables|Default|GetFireParticleSystem))
        (bind _returnvalue_3 (Effects|SpawnEmitteratLocation "/Game/StarterContent/Particles/P_Smoke.P_Smoke" (Transformation|GetWorldLocation (Variables|Default|GetScene))))
        (Utilities|FlowControl|Delay 2.0)
        (Components|Activation|Deactivate _returnvalue_3)
        (Components|DestroyComponent (Variables|Default|GetPointOfInterest_Component))
        (Default|CallExtinguish self)))
    (else
      (Utilities|FlowControl|Sequence
        (:then_0
          ;[1 1 1] 불 크기 조절
          (Utilities|FlowControl|Delay 0.1)
          (Transformation|SetWorldScale3D _scene (Math|Vector|MakeVector (+ (.x _returnvalue) _plusscaleamount) _returnvalue_2 (+ (.z _returnvalue) _plusscaleamount)))
          (Variables|Default|SetFireScale _returnvalue_2))
        (:then_1
          ;[1 1 1] 불 스폰
          (if (and (>= (Variables|Default|GetFireScale) 1.5) (Math|Boolean|Equal(Boolean) (Variables|Default|GetIsSpawned) false))
            (Utilities|FlowControl|DoOnce false
              (:Completed
                (Game|SpawnActorfromClass "BP_Fire_C" (Math|Transform|MakeTransform (Math|Vector|MakeVector (Math|Random|RandomFloatinRange (Variables|Default|GetRandomMinX) (Variables|Default|GetRandomMaxX)) (Math|Random|RandomFloatinRange (Variables|Default|GetRandomMinY) (Variables|Default|GetRandomMaxY)) (.z (Transformation|GetWorldLocation (Variables|Default|GetScene)))) "0, 0, 0" "1,1,1") "Undefined" 0 (Variables|Default|GetRandomMinY) (Variables|Default|GetRandomMaxY) (Variables|Default|GetRandomMinX) (Variables|Default|GetRandomMaxX) true 0)))))
        (:then_2
          ;[1 1 1] 불 데미지
          (if (Variables|Default|GetOnBurn)
            (Utilities|FlowControl|Delay (Variables|Default|GetIncreaseTime))
            (bind _output_get (Variables|Default|SetDamageAmount (+ (Variables|Default|GetDamageAmount) (Variables|Default|GetincreaseAmount))))
            (Default|FireDamage (Variables|Default|GetPlayer) _output_get)))))))

(event EventBeginPlay
  (Utilities|FlowControl|Sequence
    (:then_0
      (bind _returnvalue (Actor|GetActorOfClass "/Game/Blueprints/BP_FireManager.BP_FireManager_C"))
      (Utilities|IsValid _returnvalue
        (:Is%20Valid
          (Utilities|Array|AddUnique (Variables|/Game/Blueprints/BP_FireManager.BP_FireManager_C|GetArrFires _returnvalue) self)
          (EventDispatchers|BindEventtoExtinguish (EventDispatchers|CreateEvent _returnvalue :!event Extinguish)))))
    (:then_1
      (EventDispatchers|BindEventtoKillFire (delegate Custom|KillFire_Event)))
    (:then_2
      (bind _asmotion_controller_pawn (Utilities|Casting|CastToMotionControllerPawn (Game|Player|GetPlayerPawn 0)))
      (Variables|Default|SetPlayer _asmotion_controller_pawn))))

(fn ConstructionScript)