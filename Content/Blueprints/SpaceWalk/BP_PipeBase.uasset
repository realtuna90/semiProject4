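; BP_PipeBase is the base actor for a pipe repair task in the space walk section.
; On BeginPlay it registers itself with the SpaceWalkManager found in the level.
; When a BP_Pipe first leaves the Throwawaycheck volume, it broadcasts Throwaway and flags that pipe as thrown away, guarded by a DoOnce.
; Its Repair event broadcasts RepairComplete.
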(event OnComponentEndOverlap(Throwawaycheck)
  (params (OverlappedComponent :type Primitive%20Component%20Object%20Reference) (OtherActor :type Actor%20Object%20Reference) (OtherComp :type Primitive%20Component%20Object%20Reference) (OtherBodyIndex :type Integer))
  (bind _asbp_pipe (Utilities|Casting|CastToBP_Pipe OtherActor))
  (Utilities|FlowControl|DoOnce false
    (:Completed
      (Default|CallThrowaway)
      (Variables|/Game/Blueprints/SpaceWalk/BP_Pipe.BP_Pipe_C|SetThrowaway? _asbp_pipe true))))

(event Custom|Repair
  (Default|CallRepairComplete))

(event Collision|EventActorBeginOverlap
  (params (OtherActor :type Actor%20Object%20Reference)))

(event EventTick
  (params (DeltaSeconds :type Float%20%28single-precision%29)))

(event EventBeginPlay
  (bind _returnvalue (Actor|GetActorOfClass "/Game/Blueprints/SpaceWalk/SpaceWalkManager.SpaceWalkManager_C"))
  (Utilities|IsValid _returnvalue
    (:Is%20Valid
      (Variables|/Game/Blueprints/SpaceWalk/SpaceWalkManager.SpaceWalkManager_C|SetPipeBase _returnvalue self))))

(fn ConstructionScript)