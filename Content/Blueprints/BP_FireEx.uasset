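; BP_FireEx is a VR fire extinguisher that registers with BP_FireManager and attaches to the right-hand socket when equipped.
; While equipped and in use, Tick keeps a smoke emitter at TracePoint and runs a short, debug-drawn forward line trace, calling KillFire on any BP_Fire hit.
; Releasing use deactivates the smoke.
; Equipping also fires a one-time Equiped dispatcher in a specific level and manager phase.
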(event Custom|FireSmall)

(event EventBeginPlay
  (bind _returnvalue (Actor|GetActorOfClass "/Game/Blueprints/BP_FireManager.BP_FireManager_C"))
  (bind _output_get (Variables|Default|SetFireManager _returnvalue))
  (Variables|/Game/Blueprints/BP_FireManager.BP_FireManager_C|SetFireEX _output_get self))

(event EventTick
  (params (DeltaSeconds :type Float%20%28single-precision%29))
  (bind _tracepoint (Variables|Default|GetTracePoint))
  (bind _returnvalue (Transformation|GetWorldLocation _tracepoint))
  (if (Variables|Default|GetisEquipped)
    (if (Variables|Default|GetisUse)
      (Utilities|FlowControl|Sequence
        (:then_0
          (Utilities|IsValid (Variables|Default|GetSmokeParticle)
            (:Is%20Valid
              (if (not (Components|Activation|IsActive (Variables|Default|GetSmokeParticle)))
                (Components|Activation|Activate (Variables|Default|GetSmokeParticle) false)))
            (:Is%20Not%20Valid
              (bind _returnvalue_2 (Effects|SpawnEmitteratLocation "/Game/FX/P_FireExtinguishSmoke.P_FireExtinguishSmoke" (Variables|/Script/Engine.SceneComponent|GetRelativeLocation (Variables|Default|GetTracePoint)) (Variables|/Script/Engine.SceneComponent|GetRelativeRotation (Variables|Default|GetTracePoint))))
              (Utilities|IsValid (Variables|Default|GetSmokeParticle)
                (:Is%20Not%20Valid
                  (Variables|Default|SetSmokeParticle _returnvalue_2))))))
        (:then_1
          (bind _outhit (Collision|LineTraceByChannel _returnvalue (+ _returnvalue (* (Math|Vector|GetForwardVector (Transformation|GetWorldRotation _tracepoint)) 1e+02)) "TraceTypeQuery3" true 0 "ForOneFrame"))
          (bind _asbp_fire (Utilities|Casting|CastToBP_Fire (.HitActor (Collision|BreakHitResult _outhit))))
          (Utilities|FlowControl|Sequence
            (:then_0
              (Utilities|FlowControl|DoOnce false
                (:Completed
                  (EventDispatchers|BindEventtoKillFire _asbp_fire (delegate Custom|FireSmall)))))
            (:then_1
              (Utilities|IsValid _asbp_fire
                (:Is%20Valid
                  (Default|CallKillFire _asbp_fire)
                  (Utilities|FlowControl|Delay 0.1))))))
        (:then_2
          (if (Components|Activation|IsActive (Variables|Default|GetSmokeParticle))
            (Transformation|SetWorldTransform (Variables|Default|GetSmokeParticle) (Transformation|GetWorldTransform (Variables|Default|GetTracePoint)) false false))))
      (else
        (Utilities|IsValid (Variables|Default|GetSmokeParticle)
          (:Is%20Valid
            (if (Components|Activation|IsActive (Variables|Default|GetSmokeParticle))
              (Components|Activation|Deactivate (Variables|Default|GetSmokeParticle)))))))))

(event EventEquip
  (params (EquipTo :type Scene%20Component%20Object%20Reference))
  (Physics|SetSimulatePhysics (Variables|Default|GetStaticMeshComponent) false)
  (Transformation|AttachComponentToComponent (VehicleSound|GetRootComponent) EquipTo "SocketRightHand" "SnapToTarget" "SnapToTarget" "KeepWorld" true)
  (Variables|Default|SetisEquipped true)
  (bind _asvrgame_mode (Utilities|Casting|CastToVRGameMode (Game|GetGameMode)))
  (if (and (Utilities|Enum|Equal(Enum) (Variables|/Game/Blueprints/VRGameMode.VRGameMode_C|Getlevel _asvrgame_mode) "NewEnumerator0") (== (Variables|/Game/Blueprints/BP_FireManager.BP_FireManager_C|GetPhase (Variables|Default|GetFireManager)) 1))
    (Utilities|FlowControl|DoOnce false
      (:Completed
        (Default|CallEquiped)))))

(fn ConstructionScript)