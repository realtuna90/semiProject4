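; BP_FingerPrintDoor is a sliding door opened by a linked fingerprint instance.
; On BeginPlay it binds its open event to that instance; the event plays a timeline that lerps the door mesh's relative location between closed and open vectors.
; Any end overlap on ZoneTrigger reverses the timeline to close it.
; Each timeline update also restarts a door sound, using the relative vector as its world location.
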(event OnComponentEndOverlap(ZoneTrigger)
  (params (OverlappedComponent :type Primitive%20Component%20Object%20Reference) (OtherActor :type Actor%20Object%20Reference) (OtherComp :type Primitive%20Component%20Object%20Reference) (OtherBodyIndex :type Integer))
  (bind _doorposition (Timeline|Timeline_0 Reverse)
    (:Update
      (Audio|PlaySoundatLocation "/Game/SciFiPopulate/Maps/DemoLevel/Sounds/Futuristic_door.Futuristic_door" (Math|Vector|Lerp(Vector) (Variables|DoorSetup|GetDoorClose) (Variables|DoorSetup|GetDoorOpen) _doorposition) "0, 0, 0" 0.1 1.5 0.0 0 0 0)
      (Transformation|SetRelativeLocation (Variables|Default|GetSM_CConsoleSModuleB) (Math|Vector|Lerp(Vector) (Variables|DoorSetup|GetDoorClose) (Variables|DoorSetup|GetDoorOpen) _doorposition) false false) ; The new location is based on the vectors and triggered by the 'TimeLine' node
    )))

(event Custom|DoorOpen_Event
  (bind _doorposition (Timeline|Timeline_0 Play)
    (:Update
      (Audio|PlaySoundatLocation "/Game/SciFiPopulate/Maps/DemoLevel/Sounds/Futuristic_door.Futuristic_door" (Math|Vector|Lerp(Vector) (Variables|DoorSetup|GetDoorClose) (Variables|DoorSetup|GetDoorOpen) _doorposition) "0, 0, 0" 0.1 1.5 0.0 0 0 0)
      (Transformation|SetRelativeLocation (Variables|Default|GetSM_CConsoleSModuleB) (Math|Vector|Lerp(Vector) (Variables|DoorSetup|GetDoorClose) (Variables|DoorSetup|GetDoorOpen) _doorposition) false false) ; The new location is based on the vectors and triggered by the 'TimeLine' node
    )))

(event EventBeginPlay
  (bind _fingerprintinstance (Variables|Default|GetFingerPrintInstance))
  (Utilities|IsValid _fingerprintinstance
    (:Is%20Valid
      (EventDispatchers|BindEventtoOpenDoor _fingerprintinstance (delegate Custom|DoorOpen_Event)))))

(fn ConstructionScript)