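; BP_DriverGun is an equippable driver tool that pulls out BP_Screw actors with a forward beam.
; While equipped and in use, Tick line-traces from TracePoint, binds Screw to a new target's PullOut, then calls PullOut on subsequent ticks.
; The Screw callback flags a hit, clips the spline-mesh beam to the impact and spawns sparks.
; Paired DoOnce nodes that reset each other toggle drill and spark sounds only on state changes.
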(event Custom|Screw
  (bind _traceend (Variables|Default|GetTraceEnd))
  (bind _output_get (Variables|Default|SetonHit (.bBlockingHit (Collision|BreakHitResult (stale EventTick _outhit)))))
  (Transformation|SetWorldLocation _traceend (.Location (Collision|BreakHitResult (stale EventTick _outhit))) false false)
  (SplineMesh|SetEndPosition (Variables|Default|GetSplineMesh) (Variables|/Script/Engine.SceneComponent|GetRelativeLocation _traceend) _output_get)
  (Effects|SpawnEmitteratLocation "/Game/FX/P_DriverSpark.P_DriverSpark" (.Location (Collision|BreakHitResult (stale EventTick _outhit))) "0, 0, 0" "0.100000,0.100000,0.100000"))

(event EventTick
  (params (DeltaSeconds :type Float%20%28single-precision%29))
  (bind _tracepoint (Variables|Default|GetTracePoint))
  (bind _sparksound (Variables|Default|GetSparkSound))
  (bind _isuse (Variables|Default|GetisUse))
  (bind _tracepoint_2 (Variables|Default|GetTracePoint))
  (bind _splinemesh (Variables|Default|GetSplineMesh))
  (bind _returnvalue (Transformation|GetWorldLocation _tracepoint))
  (bind _relativelocation (Variables|/Script/Engine.SceneComponent|GetRelativeLocation _tracepoint_2))
  (Variables|Default|SetonHit false)
  (if (Variables|Default|GetisEquipped)
    (if _isuse
      (Utilities|FlowControl|Sequence
        (:then_0
          (bind _outhit (Collision|LineTraceByChannel _returnvalue (+ _returnvalue (* (Math|Vector|GetForwardVector (Transformation|GetWorldRotation _tracepoint)) 1e+03)) "TraceTypeQuery3" true 0 "None"))
          (bind _asbp_screw (Utilities|Casting|CastToBP_Screw (.HitActor (Collision|BreakHitResult _outhit))))
          (if (or (Math|Boolean|Equal(Boolean) (Utilities|IsValid (Variables|Default|GetcurTarrget)) false) (!= (Variables|Default|GetcurTarrget) _asbp_screw))
            (Variables|Default|SetcurTarrget _asbp_screw)
            (EventDispatchers|BindEventtoPullOut _asbp_screw (delegate Custom|Screw))
            (else
              (Default|CallPullOut _asbp_screw))))
        (:then_1
          (if (Math|Boolean|Equal(Boolean) (Variables|Default|GetonHit) false)
            (SplineMesh|SetStartandEnd _splinemesh _relativelocation "0, 0, 0" (+ _relativelocation (* (Math|Vector|GetForwardVector (Variables|/Script/Engine.SceneComponent|GetRelativeRotation _tracepoint_2)) 1e+03)) "0, 0, 0" true :!class /Script/Engine.SplineMeshComponent)
            (Rendering|SetVisibility _splinemesh true false)))
        (:then_2
          (if _isuse :!label _label
            (Utilities|FlowControl|DoOnce false :!label _label_2
              (:Completed
                (Components|Activation|Activate (Variables|Default|Get드릴_Cue) false)
                (goto _label_3 Reset)))
            (else
              (Utilities|FlowControl|DoOnce false :!label _label_3
                (:Completed
                  (Components|Activation|Deactivate (Variables|Default|Get드릴_Cue))
                  (goto _label_2 Reset))))))
        (:then_3
          (if (Variables|Default|GetonHit)
            (Utilities|FlowControl|DoOnce false :!label _label_4
              (:Completed
                (Transformation|SetWorldLocation _sparksound (Transformation|GetWorldLocation (Variables|Default|GetTraceEnd)) false false)
                (Components|Activation|Activate _sparksound false)
                (goto _label_5 Reset)))
            (else
              (Utilities|FlowControl|DoOnce false :!label _label_5
                (:Completed
                  (Components|Activation|Deactivate (Variables|Default|GetSparkSound))
                  (goto _label_4 Reset)))))))
      (else
        (Utilities|FlowControl|Sequence
          (:then_0
            (Rendering|SetVisibility (Variables|Default|GetSplineMesh) false false)
            (goto _label))
          (:then_1
            (goto _label_5)))))))

(fn ConstructionScript
  (Variables|Default|SetHighLightMesh 0))