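; BP_Door2 is a two-panel sliding door that opens on DoorOpen_Event and closes automatically.
; A timeline moves the panels in opposite directions between DoorClose and DoorOpen and plays a futuristic door sound.
; Tick counts down the open time, resetting it while the sensor is overlapped.
; Close polls with zero-length Delay loops until the countdown ends and no MotionControllerPawn occupies ZoneTrigger, then reverses the timeline.
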(event Custom|DoorOpen_Event
  (params (Sensor :type BP%20Finger%20Print%20Gas%20Room%20Object%20Reference))
  (Variables|Default|SetIsOpen true)
  (Variables|Default|SetopenTime 4.25)
  (bind _doorposition (Timeline|타임라인_0 Play)
    (:Update
      (Utilities|FlowControl|Sequence
        (:then_0
          (Transformation|SetRelativeLocation (Variables|Default|GetStaticMeshComponent1) (Math|Vector|Lerp(Vector) (Variables|Default|GetDoorClose) (Variables|Default|GetDoorOpen) _doorposition) false false) ; The new location is based on the vectors and triggered by the 'TimeLine' node
        )
        (:then_1
          (Transformation|SetRelativeLocation (Variables|Default|GetStaticMeshComponent0) (Math|Vector|Lerp(Vector) (Variables|Default|GetDoorClose) (* (Variables|Default|GetDoorOpen) -1.0) _doorposition) false false) ; The new location is based on the vectors and triggered by the 'TimeLine' node
        )))
    (:Finished
      (if (Variables|Default|GetIsOpen)
        (CallFunction|Close)))
    (:SoundTiming
      (Audio|PlaySoundatLocation "/Game/SciFiPopulate/Maps/DemoLevel/Sounds/Futuristic_door.Futuristic_door" (Transformation|GetActorLocation) "0, 0, 0" 0.1 1.5 0.0 0 0 0))))

(event Custom|close
  (if (or (Variables|Default|GetIsOpen) (!= (Utilities|Array|Length (Collision|GetOverlappingActors (Variables|Default|GetZoneTrigger) "/Game/Blueprints/MotionControllerPawn.MotionControllerPawn_C" :!class /Script/Engine.PrimitiveComponent)) 0)) :!label _label
    (Utilities|FlowControl|Delay 0.0)
    (goto _label)
    (else
      (bind _doorposition (Timeline|타임라인_0 Reverse)
        (:Update
          (Utilities|FlowControl|Sequence
            (:then_0
              (Transformation|SetRelativeLocation (Variables|Default|GetStaticMeshComponent1) (Math|Vector|Lerp(Vector) (Variables|Default|GetDoorClose) (Variables|Default|GetDoorOpen) _doorposition) false false) ; The new location is based on the vectors and triggered by the 'TimeLine' node
            )
            (:then_1
              (Transformation|SetRelativeLocation (Variables|Default|GetStaticMeshComponent0) (Math|Vector|Lerp(Vector) (Variables|Default|GetDoorClose) (* (Variables|Default|GetDoorOpen) -1.0) _doorposition) false false) ; The new location is based on the vectors and triggered by the 'TimeLine' node
            )))
        (:Finished
          (if (Variables|Default|GetIsOpen)
            (CallFunction|Close)))
        (:SoundTiming
          (Audio|PlaySoundatLocation "/Game/SciFiPopulate/Maps/DemoLevel/Sounds/Futuristic_door.Futuristic_door" (Transformation|GetActorLocation) "0, 0, 0" 0.1 1.5 0.0 0 0 0))))))

(event EventTick
  (params (DeltaSeconds :type Float%20%28single-precision%29))
  (if (Variables|Default|GetIsOpen)
    (if (Variables|/Game/Blueprints/GasEvent/BP_FingerPrintGasRoom.BP_FingerPrintGasRoom_C|GetIs%20Overlap (stale Custom|DoorOpen_Event Sensor)) :!label _label
      (Variables|Default|SetopenTime 4.0)
      (Utilities|FlowControl|Delay 0.0)
      (goto _label)
      (elif (< (- (Variables|Default|GetopenTime) DeltaSeconds) 0.0)
        (Variables|Default|SetIsOpen false)
        (else
          (Variables|Default|SetopenTime (- (Variables|Default|GetopenTime) DeltaSeconds)))))))

(fn ConstructionScript)