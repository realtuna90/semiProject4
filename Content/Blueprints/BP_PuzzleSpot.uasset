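; BP_PuzzleSpot is a colored connection point, parented to BP_SpherePuzzle, in a color-pair matching puzzle.
; The puzzle's start event enables its collision and whitens it; interacting with a first spot stores its color and reference on the sphere.
; A second spot of the same color turns both blue and reveals that color's line, while a mismatch resets the first.
; Tick also resets the pending spot when the interacting Gun stops being used.
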(event Custom|PuzzleStart
  (params (Controller :type BP%20Motion%20Controller%20Object%20Reference))
  (Variables|Default|SetFingertip (Variables|/Game/Blueprints/BP_MotionController.BP_MotionController_C|GetFingertip Controller))
  (Collision|SetCollisionEnabled (Variables|Default|GetSphereCollision) "QueryAndPhysics")
  (CallFunction|SetMaterial "/Engine/SP_Puzzle_White.SP_Puzzle_White"))

(event Custom|커스텀이벤트_1
  (params (Gun :type BP%20Puzzle%20Gun%20Object%20Reference))
  (bind _puzzlesphere (Variables|Default|GetPuzzleSphere))
  (bind _puzzlesphere_2 (Variables|Default|GetPuzzleSphere))
  (bind _puzzlesphere_3 (Variables|Default|GetPuzzleSphere))
  (Utilities|FlowControl|Sequence
    (:then_0
      (Utilities|FlowControl|DoOnce false
        (:Completed
          (Variables|Default|SetGun Gun))))
    (:then_1
      (if (Utilities|Text|TextIsEmpty (Variables|/Game/Blueprints/BP_SpherePuzzle.BP_SpherePuzzle_C|GetNowColor (Variables|Default|GetPuzzleSphere)))
        (if (Utilities|Enum|Equal(Enum) (Variables|Default|GetColor) (Utilities|Text|MakeLiteralText "Red"))
          (CallFunction|SetMaterial "/Engine/EngineResources/Sp_Puzzle_red.Sp_Puzzle_red")
          (Variables|/Game/Blueprints/BP_SpherePuzzle.BP_SpherePuzzle_C|SetNowColor _puzzlesphere_3 (Variables|Default|GetColor) :!label _label)
          (Collision|SetCollisionEnabled (Variables|Default|GetSphereCollision) "NoCollision")
          (Variables|/Game/Blueprints/BP_SpherePuzzle.BP_SpherePuzzle_C|SetNowSpot _puzzlesphere_3 self)
          (elif (Utilities|Enum|Equal(Enum) (Variables|Default|GetColor) (Utilities|Text|MakeLiteralText "Yellow"))
            (CallFunction|SetMaterial "/Engine/SP_Puzzle_Yellow.SP_Puzzle_Yellow")
            (goto _label)
            (elif (Utilities|Enum|Equal(Enum) (Variables|Default|GetColor) (Utilities|Text|MakeLiteralText "Green"))
              (CallFunction|SetMaterial "/Engine/SP_Puzzle_Green.SP_Puzzle_Green")
              (goto _label))))
        (elif (Utilities|Enum|Equal(Enum) (Variables|/Game/Blueprints/BP_SpherePuzzle.BP_SpherePuzzle_C|GetNowColor (Variables|Default|GetPuzzleSphere)) (Variables|Default|GetColor))
          (CallFunction|SetMaterial (Variables|/Game/Blueprints/BP_SpherePuzzle.BP_SpherePuzzle_C|GetNowSpot _puzzlesphere_2) "/Engine/SP_Puzzle_Blue.SP_Puzzle_Blue")
          (CallFunction|SetMaterial "/Engine/SP_Puzzle_Blue.SP_Puzzle_Blue")
          (if (Utilities|Enum|Equal(Enum) (Variables|/Game/Blueprints/BP_SpherePuzzle.BP_SpherePuzzle_C|GetNowColor _puzzlesphere) (Utilities|Text|MakeLiteralText "Red"))
            (Rendering|SetVisibility (Variables|/Game/Blueprints/BP_SpherePuzzle.BP_SpherePuzzle_C|GetLine_Red _puzzlesphere) true false)
            (Variables|/Game/Blueprints/BP_SpherePuzzle.BP_SpherePuzzle_C|SetNowColor _puzzlesphere_2 "" :!label _label_2)
            (Collision|SetCollisionEnabled (Variables|Default|GetSphereCollision) "NoCollision")
            (bind _asbp_sphere_puzzle (Utilities|Casting|CastToBP_SpherePuzzle (Variables|Default|GetPuzzleSphere)))
            (Variables|/Game/Blueprints/BP_SpherePuzzle.BP_SpherePuzzle_C|SetNowSpot _asbp_sphere_puzzle 0)
            (elif (Utilities|Enum|Equal(Enum) (Variables|/Game/Blueprints/BP_SpherePuzzle.BP_SpherePuzzle_C|GetNowColor _puzzlesphere) (Utilities|Text|MakeLiteralText "Yellow"))
              (Rendering|SetVisibility (Variables|/Game/Blueprints/BP_SpherePuzzle.BP_SpherePuzzle_C|GetLine_Yellow _puzzlesphere) true false)
              (goto _label_2)
              (elif (Utilities|Enum|Equal(Enum) (Variables|/Game/Blueprints/BP_SpherePuzzle.BP_SpherePuzzle_C|GetNowColor _puzzlesphere) (Utilities|Text|MakeLiteralText "Green"))
                (Rendering|SetVisibility (Variables|/Game/Blueprints/BP_SpherePuzzle.BP_SpherePuzzle_C|GetLine_Green _puzzlesphere) true false)
                (goto _label_2))))
          (else
            (CallFunction|SetMaterial (Variables|/Game/Blueprints/BP_SpherePuzzle.BP_SpherePuzzle_C|GetNowSpot _puzzlesphere_2) "/Engine/SP_Puzzle_White.SP_Puzzle_White")
            (Variables|/Game/Blueprints/BP_SpherePuzzle.BP_SpherePuzzle_C|SetNowColor _puzzlesphere_2 "")
            (Collision|SetCollisionEnabled (Variables|BP_PuzzleSpot_C|GetSphereCollision (Variables|/Game/Blueprints/BP_SpherePuzzle.BP_SpherePuzzle_C|GetNowSpot _puzzlesphere_2)) "QueryAndPhysics")))))))

(event EventBeginPlay
  (EventDispatchers|BindEventtoStartPuzzle (Variables|Default|GetPuzzleSphere) (delegate Custom|PuzzleStart))
  (Variables|Default|SetInitialLocation (Transformation|GetActorLocation))
  (EventDispatchers|BindEventtoInteraction (delegate Custom|커스텀이벤트_1)))

(event EventTick
  (params (DeltaSeconds :type Float%20%28single-precision%29))
  (bind _gun (Variables|Default|GetGun))
  (bind _puzzlesphere (Variables|Default|GetPuzzleSphere))
  (bind _nowspot (Variables|/Game/Blueprints/BP_SpherePuzzle.BP_SpherePuzzle_C|GetNowSpot _puzzlesphere))
  (Utilities|IsValid _gun
    (:Is%20Valid
      (Utilities|IsValid (Variables|/Game/Blueprints/BP_SpherePuzzle.BP_SpherePuzzle_C|GetNowSpot (Variables|Default|GetPuzzleSphere))
        (:Is%20Valid
          (if (not (Variables|/Game/Blueprints/BP_Equipment.BP_Equipment_C|GetisUse _gun))
            (CallFunction|SetMaterial _nowspot "/Engine/SP_Puzzle_White.SP_Puzzle_White")
            (Variables|/Game/Blueprints/BP_SpherePuzzle.BP_SpherePuzzle_C|SetNowColor _puzzlesphere "")
            (Collision|SetCollisionEnabled (Variables|BP_PuzzleSpot_C|GetSphereCollision _nowspot) "QueryAndPhysics")))))))

(fn ConstructionScript
  (bind _returnvalue (Actor|GetParentActor))
  (CallFunction|SetMaterial (Variables|Default|GetMaterial))
  (Utilities|IsValid _returnvalue
    (:Is%20Valid
      (bind _asbp_sphere_puzzle (Utilities|Casting|CastToBP_SpherePuzzle _returnvalue))
      (Variables|Default|SetPuzzleSphere _asbp_sphere_puzzle))))

(fn SetMaterial
  (params (Material :type Material%20Interface%20Object%20Reference))
  (Rendering|Material|SetMaterial (Variables|Default|GetPlane) 0 Material))