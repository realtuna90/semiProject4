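; Fingerprint scanner actor for the gas room that opens a door when a motion controller touches it.
; On BeginPlay it caches a BP_Door2 instance found by class lookup.
; A BP_MotionController entering the Box turns the FingerPrint screen green, sets IsOverlap and calls the door's open event with itself.
; Leaving restores the blue screen and clears the flag without closing the door.
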(event OnComponentBeginOverlap(Box)
  (params (OverlappedComponent :type Primitive%20Component%20Object%20Reference) (OtherActor :type Actor%20Object%20Reference) (OtherComp :type Primitive%20Component%20Object%20Reference) (OtherBodyIndex :type Integer) (bFromSweep :type Boolean) (SweepResult :type Hit%20Result%20Structure%20%28by%20ref%29))
  (Utilities|IsValid OverlappedComponent
    (:Is%20Valid
      (Utilities|Casting|CastToBP_MotionController OtherActor)
      (Variables|Default|SetIs%20Overlap true)
      (Rendering|Material|SetMaterial (Variables|Default|GetFingerPrint) 1 "/Game/2Materials/Screen_Green.Screen_Green")
      (Default|DoorOpenEvent (Variables|Default|GetDoor) self))))

(event OnComponentEndOverlap(Box)
  (params (OverlappedComponent :type Primitive%20Component%20Object%20Reference) (OtherActor :type Actor%20Object%20Reference) (OtherComp :type Primitive%20Component%20Object%20Reference) (OtherBodyIndex :type Integer))
  (Utilities|IsValid OverlappedComponent
    (:Is%20Valid
      (Utilities|Casting|CastToBP_MotionController OtherActor)
      (Rendering|Material|SetMaterial (Variables|Default|GetFingerPrint) 1 "/Game/2Materials/Screen_Blue.Screen_Blue")
      (Variables|Default|SetIs%20Overlap false))))

(event EventBeginPlay
  (bind _returnvalue (Actor|GetActorOfClass "/Game/Blueprints/GasEvent/BP_Door2.BP_Door2_C"))
  (Variables|Default|SetDoor _returnvalue))

(fn ConstructionScript)