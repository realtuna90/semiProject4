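; BP_Valve is a VR valve that the player grabs and twists with a motion controller.
; While held, Tick projects the hand's right vector onto the valve's plane and applies frame-to-frame rotation deltas to the mesh, blocking further turns past either yaw limit.
; Accumulated rotation lowers the audio volume.
; Reaching the upper limit once plays an explosion sound and shoves the player's physics root opposite camera forward, with temporary linear damping.
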(event EventTick
  (params (DeltaSeconds :type Float%20%28single-precision%29))
  (Utilities|FlowControl|Sequence
    (:then_0
      (if (Variables|Default|GetIsUse)
        (if (<= (Variables|Default|GetRotateValue) -5e+01)
          (if (>= (.Yaw (Math|Rotator|BreakRotator (Math|Rotator|Delta(Rotator) (Math|Rotator|FindLookatRotation (Math|Vector|MakeVector 0.0 0.0 0.0) (Math|Vector|Normalize (Math|Vector|ProjectVectorontoPlane (Math|Vector|GetRightVector (Variables|/Game/Blueprints/BP_MotionController.BP_MotionController_C|GetHandMesh (stale EventPickup MotionController))) (Transformation|GetActorUpVector)))) (Variables|Default|GetNowRotation)))) 0.0)
            (Transformation|AddRelativeRotation (Variables|Default|GetStaticMesh) (Math|Rotator|Delta(Rotator) (Math|Rotator|FindLookatRotation (Math|Vector|MakeVector 0.0 0.0 0.0) (Math|Vector|Normalize (Math|Vector|ProjectVectorontoPlane (Math|Vector|GetRightVector (Variables|/Game/Blueprints/BP_MotionController.BP_MotionController_C|GetHandMesh (stale EventPickup MotionController))) (Transformation|GetActorUpVector)))) (Variables|Default|GetNowRotation)) false false :!label _label)
            (Variables|Default|SetRotateValue (+ (.Yaw (Math|Rotator|BreakRotator (Math|Rotator|Delta(Rotator) (Math|Rotator|FindLookatRotation (Math|Vector|MakeVector 0.0 0.0 0.0) (Math|Vector|Normalize (Math|Vector|ProjectVectorontoPlane (Math|Vector|GetRightVector (Variables|/Game/Blueprints/BP_MotionController.BP_MotionController_C|GetHandMesh (stale EventPickup MotionController))) (Transformation|GetActorUpVector)))) (Variables|Default|GetNowRotation)))) (Variables|Default|GetRotateValue)))
            (Variables|Default|SetNowRotation (Math|Rotator|FindLookatRotation (Math|Vector|MakeVector 0.0 0.0 0.0) (Math|Vector|Normalize (Math|Vector|ProjectVectorontoPlane (Math|Vector|GetRightVector (Variables|/Game/Blueprints/BP_MotionController.BP_MotionController_C|GetHandMesh (stale EventPickup MotionController))) (Transformation|GetActorUpVector))))))
          (elif (>= (Variables|Default|GetRotateValue) 2.5e+02)
            (if (<= (.Yaw (Math|Rotator|BreakRotator (Math|Rotator|Delta(Rotator) (Math|Rotator|FindLookatRotation (Math|Vector|MakeVector 0.0 0.0 0.0) (Math|Vector|Normalize (Math|Vector|ProjectVectorontoPlane (Math|Vector|GetRightVector (Variables|/Game/Blueprints/BP_MotionController.BP_MotionController_C|GetHandMesh (stale EventPickup MotionController))) (Transformation|GetActorUpVector)))) (Variables|Default|GetNowRotation)))) 0.0)
              (goto _label))
            (else
              (goto _label))))))
    (:then_2
      (if (>= (Variables|Default|GetRotateValue) 2.5e+02)
        (Utilities|FlowControl|DoOnce false
          (:Completed
            (bind _asmotion_controller_pawn (Utilities|Casting|CastToMotionControllerPawn (Game|Player|GetPlayerPawn 0)))
            (Physics|AddImpulse (Variables|/Game/Blueprints/MotionControllerPawn.MotionControllerPawn_C|GetPhysicsRoot _asmotion_controller_pawn) (* (Math|Vector|GetForwardVector (Variables|/Game/Blueprints/MotionControllerPawn.MotionControllerPawn_C|GetCamera _asmotion_controller_pawn)) -3e+01) "None" false)
            (Audio|PlaySoundatLocation "/Game/4Sound/폭발소리.폭발소리" (Transformation|GetActorLocation) "0, 0, 0" 1.0 1.0 0.0 0 0 0)
            (Class|PrimitiveComponent|SetLinearDamping (Variables|/Game/Blueprints/MotionControllerPawn.MotionControllerPawn_C|GetPhysicsRoot _asmotion_controller_pawn) 2.0)
            (Utilities|FlowControl|Delay 2.0)
            (Class|PrimitiveComponent|SetLinearDamping (Variables|/Game/Blueprints/MotionControllerPawn.MotionControllerPawn_C|GetPhysicsRoot _asmotion_controller_pawn) 0.0)))))
    (:then_3
      (Audio|Components|Audio|SetVolumeMultiplier (Variables|Default|GetAudio) (+ (* (Variables|Default|GetRotateValue) -0.01) 2.5) :!class /Script/Engine.AudioComponent))))

(event EventPickup
  (params (AttachTo :type Scene%20Component%20Object%20Reference) (MotionController :type BP%20Motion%20Controller%20Object%20Reference))
  (Variables|Default|SetIsUse true)
  (Variables|Default|SetNowRotation (Math|Rotator|FindLookatRotation (Math|Vector|MakeVector 0.0 0.0 0.0) (Math|Vector|Normalize (Math|Vector|ProjectVectorontoPlane (Math|Vector|GetRightVector (Variables|/Game/Blueprints/BP_MotionController.BP_MotionController_C|GetHandMesh MotionController)) (Transformation|GetActorUpVector))))))

(event EventDrop
  (Variables|Default|SetIsUse false))

(fn ConstructionScript)