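; BP_GasManager is the stage manager for the gas room event, driving its phases through to stage clear.
; It hides BP_GasRoom until "outside_3" unloads, then reveals it and enables its collision if the VRGameMode level matches this stage.
; The first BP_Biotank break and the Module's GetModule event advance Phase.
; Zero-delay loops poll Phase to notify VRGameMode, bind the module event and trigger the stage change.
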(event Custom|biobreak
  (Utilities|FlowControl|DoOnce false
    (:Completed
      (Math|Integer|IncrementInt (Variables|Default|GetPhase)))))

(event Custom|StageClear
  ;[1 1 1] 스테이지 클리어
  (bind _asvrgame_mode (Utilities|Casting|CastToVRGameMode (Game|GetGameMode)))
  (Default|StageChange _asvrgame_mode (Variables|Default|GetstageNum)))

(event Custom|GetModule
  (Math|Integer|IncrementInt (Variables|Default|GetPhase)))

(event Custom|커스텀이벤트_0
  (bind _returnvalue (Game|GetGameMode))
  (bind _gasroom (Variables|Default|GetgasRoom))
  (bind _asvrgame_mode (Utilities|Casting|CastToVRGameMode _returnvalue))
  (if (Utilities|Enum|Equal(Enum) (Variables|/Game/Blueprints/VRGameMode.VRGameMode_C|Getlevel _asvrgame_mode) (Variables|Default|GetstageNum))
    (bind _asvrgame_mode_2 (Utilities|Casting|CastToVRGameMode _returnvalue))
    (Default|CallOnChangePhase _asvrgame_mode_2 (Variables|Default|GetstageNum) (Variables|Default|GetPhase))
    (Utilities|FlowControl|Sequence
      (:then_0
        (Rendering|SetActorHiddenInGame _gasroom false)
        (Collision|SetCollisionEnabled (Variables|/Game/Blueprints/GasEvent/BP_GasRoom.BP_GasRoom_C|GetBox _gasroom) "QueryAndPhysics")
        (if (== (Variables|Default|GetPhase) 2) :!label _label
          (bind _asvrgame_mode_3 (Utilities|Casting|CastToVRGameMode (Game|GetGameMode)))
          (Default|CallOnChangePhase _asvrgame_mode_3 (Variables|Default|GetstageNum) (Variables|Default|GetPhase))
          (EventDispatchers|BindEventtoGetModule (Variables|Default|GetModule) (delegate Custom|GetModule))
          (else
            (Utilities|FlowControl|Delay 0.0)
            (goto _label))))
      (:then_1
        (if (== (Variables|Default|GetPhase) 3) :!label _label_2
          (CallFunction|StageClear)
          (else
            (Utilities|FlowControl|Delay 0.0)
            (goto _label_2)))))))

(event Custom|커스텀이벤트_1
  (params (curStage :type LevelEnum%20Enum :default "NewEnumerator4"))
  (bind _returnvalue (Game|GetGameMode))
  (bind _gasroom (Variables|Default|GetgasRoom))
  (Development|PrintString "Hello")
  (bind _asvrgame_mode (Utilities|Casting|CastToVRGameMode _returnvalue))
  (if (Utilities|Enum|Equal(Enum) (Variables|/Game/Blueprints/VRGameMode.VRGameMode_C|Getlevel _asvrgame_mode) (Variables|Default|GetstageNum))
    (bind _asvrgame_mode_2 (Utilities|Casting|CastToVRGameMode _returnvalue))
    (Default|CallOnChangePhase _asvrgame_mode_2 (Variables|Default|GetstageNum) (Variables|Default|GetPhase))
    (Utilities|FlowControl|Sequence
      (:then_0
        (Rendering|SetActorHiddenInGame _gasroom false)
        (Collision|SetCollisionEnabled (Variables|/Game/Blueprints/GasEvent/BP_GasRoom.BP_GasRoom_C|GetBox _gasroom) "QueryAndPhysics")
        (if (== (Variables|Default|GetPhase) 2) :!label _label
          (bind _asvrgame_mode_3 (Utilities|Casting|CastToVRGameMode (Game|GetGameMode)))
          (Default|CallOnChangePhase _asvrgame_mode_3 (Variables|Default|GetstageNum) (Variables|Default|GetPhase))
          (EventDispatchers|BindEventtoGetModule (Variables|Default|GetModule) (delegate Custom|GetModule))
          (else
            (Utilities|FlowControl|Delay 0.0)
            (goto _label))))
      (:then_1
        (if (== (Variables|Default|GetPhase) 3) :!label _label_2
          (CallFunction|StageClear)
          (else
            (Utilities|FlowControl|Delay 0.0)
            (goto _label_2)))))))

(event EventBeginPlay
  (Utilities|FlowControl|Sequence
    (:then_0
      (bind _returnvalue (Actor|GetActorOfClass "/Game/Blueprints/GasEvent/BP_GasRoom.BP_GasRoom_C"))
      (bind _output_get (Variables|Default|SetgasRoom _returnvalue))
      (Rendering|SetActorHiddenInGame _output_get true)
      (Collision|SetCollisionEnabled (Variables|/Game/Blueprints/GasEvent/BP_GasRoom.BP_GasRoom_C|GetBox _output_get) "NoCollision")
      (bind _outactors (Actor|GetAllActorsOfClass "/Game/Blueprints/GasEvent/BP_Biotank.BP_Biotank_C"))
      (for _array_element _outactors
        (EventDispatchers|BindEventtoDestruct _array_element (delegate Custom|biobreak))))
    (:then_1
      (EventDispatchers|BindEventtoOnLevelUnloaded (Class|GameplayStatics|GetStreamingLevel "outside_3") (delegate Custom|커스텀이벤트_0)))))

(fn ConstructionScript)