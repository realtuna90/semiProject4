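; Fire stage manager that spawns fires when the VR game mode switches to its stage number.
; A spawn routine creates BP_Fire actors at random points within X/Y bounds at a fixed height.
; Extinguish removes a fire from the tracked array and destroys it, advancing the game mode's stage once the array is empty.
; A helper toggles BP_HighLight child actors attached to a target.
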(event Custom|StageClear
  ;[1 1 1] 스테이지 클리어
  (bind _asvrgame_mode (Utilities|Casting|CastToVRGameMode (Game|GetGameMode)))
  (Default|StageChange _asvrgame_mode (Variables|Default|GetstageNum)))

(event Custom|StageStart
  (params (curStage :type LevelEnum%20Enum :default "NewEnumerator3"))
  (if (Utilities|Enum|Equal(Enum) curStage (Variables|Default|GetstageNum))
    (Utilities|FlowControl|Sequence
      (:then_0
        (Utilities|FireSpawnStart
          (:Do
            (if (not (Variables|Default|GetClear?)) :!label _label
              (Utilities|FlowControl|Delay 0.0)
              (goto _label))))))))

(event EventBeginPlay
  (bind _asvrgame_mode (Utilities|Casting|CastToVRGameMode (Game|GetGameMode)))
  (EventDispatchers|BindEventtoOnChangeStage _asvrgame_mode (delegate Custom|StageStart)))

(fn ConstructionScript)

(fn Extinguish
  (params (Fire :type BP%20Fire%20Object%20Reference))
  (bind _arrfires (Variables|Default|GetArrFires))
  (Utilities|Array|RemoveIndex _arrfires (Utilities|Array|FindItem _arrfires Fire))
  (Actor|DestroyActor Fire)
  (if (< (Utilities|Array|Length (Variables|Default|GetArrFires)) 1)
    (CallFunction|StageClear)))

(fn HighLightIntersection
  (params (Target :type Actor%20Object%20Reference) (On? :type Boolean))
  (bind _array_element (Utilities|Array|ForEachLoopwithBreak (Actor|GetAllChildActors Target true))
    (:LoopBody
      (bind _asbp_high_light (Utilities|Casting|CastToBP_HighLight _array_element))
      (if (== Target (Actor|GetAttachParentActor _asbp_high_light))
        (if On?
          (Default|HighLighton _asbp_high_light false)
          (else
            (Default|HighLightOff _asbp_high_light)))))))