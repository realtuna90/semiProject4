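; BP_DriveModule is a grabbable VR module that slots into a BP_ModuleBase as part of the 2D puzzle.
; On BeginPlay it finds the base and registers itself with the 2DPuzzleManager.
; BP_MotionController pickup disables physics and attaches the mesh to the hand.
; Dropping it inside the base's box reveals the base's module mesh, fires the Input dispatcher and destroys this actor; otherwise physics resumes and it detaches.
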(event EventPickup
  (params (AttachTo :type Scene%20Component%20Object%20Reference) (MotionController :type BP%20Motion%20Controller%20Object%20Reference))
  (bind _module (Variables|Default|GetModule))
  (Physics|SetSimulatePhysics _module false)
  (Transformation|AttachComponentToComponent _module AttachTo "None" "KeepWorld" "KeepWorld" "KeepWorld" false))

(event EventBeginPlay
  (bind _returnvalue (Actor|GetActorOfClass "/Game/Blueprints/2Dpuzzle/BP_ModuleBase.BP_ModuleBase_C"))
  (Utilities|IsValid _returnvalue
    (:Is%20Valid
      (Variables|Default|SetBase _returnvalue)
      (bind _returnvalue_2 (Actor|GetActorOfClass "/Game/Blueprints/2Dpuzzle/2DPuzzleManager.2DPuzzleManager_C"))
      (Variables|/Game/Blueprints/2Dpuzzle/2DPuzzleManager.2DPuzzleManager_C|SetModule _returnvalue_2 self))))

(event EventDrop
  (if (== (Utilities|Array|Length (Collision|GetOverlappingActors (Variables|/Game/Blueprints/2Dpuzzle/BP_ModuleBase.BP_ModuleBase_C|GetBox (Variables|Default|GetBase)) "BP_DriveModule_C" :!class /Script/Engine.PrimitiveComponent)) 1)
    (Rendering|SetVisibility (Variables|/Game/Blueprints/2Dpuzzle/BP_ModuleBase.BP_ModuleBase_C|GetModule (Variables|Default|GetBase)) true false)
    (Default|CallInput)
    (Actor|DestroyActor)
    (else
      (Physics|SetSimulatePhysics (Variables|Default|GetModule) true)
      (Transformation|DetachFromActor "KeepWorld" "KeepWorld" "KeepWorld"))))

(fn ConstructionScript)