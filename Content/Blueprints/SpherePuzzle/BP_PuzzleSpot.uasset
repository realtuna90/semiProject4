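; A colored endpoint spot in the sphere puzzle, activated with the laser gun to link same-colored pairs.
; The first spot hit stores its color and itself on the parent BP_SpherePuzzle and recolors the gun's beam.
; A matching second spot draws that color's blue spline-mesh line between them and flags the color done.
; A mismatch, or Tick finding the gun no longer in use, resets the pending spot and beam to white.
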(event Custom|PuzzleStart
  (params (Controller :type BP%20Motion%20Controller%20Object%20Reference))
  (Collision|SetCollisionEnabled (Variables|Default|GetSphereCollision) "QueryAndPhysics")
  (CallFunction|SetMaterial "/Game/0Mesh/PuzzleSpotWhite.PuzzleSpotWhite"))

(event Custom|커스텀이벤트_1
  (params (Gun :type BP%20Puzzle%20Gun%20Object%20Reference))
  (bind _puzzlesphere (Variables|Default|GetPuzzleSphere))
  (bind _puzzlesphere_2 (Variables|Default|GetPuzzleSphere))
  (bind _puzzlesphere_3 (Variables|Default|GetPuzzleSphere))
  (bind _puzzlesphere_4 (Variables|Default|GetPuzzleSphere))
  (bind _line_red (Variables|/Game/Blueprints/SpherePuzzle/BP_SpherePuzzle.BP_SpherePuzzle_C|GetLine_Red _puzzlesphere))
  (bind _line_yellow (Variables|/Game/Blueprints/SpherePuzzle/BP_SpherePuzzle.BP_SpherePuzzle_C|GetLine_Yellow _puzzlesphere))
  (bind _line_green (Variables|/Game/Blueprints/SpherePuzzle/BP_SpherePuzzle.BP_SpherePuzzle_C|GetLine_Green _puzzlesphere))
  (bind _returnvalue (Transformation|GetWorldTransform _line_green))
  (bind _returnvalue_2 (Transformation|GetWorldTransform _line_red))
  (bind _returnvalue_3 (Transformation|GetWorldTransform _line_yellow))
  (Utilities|FlowControl|Sequence
    (:then_0
      (Utilities|FlowControl|DoOnce false
        (:Completed
          (Variables|Default|SetGun Gun))))
    (:then_1
      (if (Utilities|Text|TextIsEmpty (Variables|/Game/Blueprints/SpherePuzzle/BP_SpherePuzzle.BP_SpherePuzzle_C|GetNowColor (Variables|Default|GetPuzzleSphere)))
        (if (Utilities|Enum|Equal(Enum) (Variables|Default|GetColor) (Utilities|Text|MakeLiteralText "Red"))
          (CallFunction|SetMaterial "/Game/0Mesh/PuzzleSpotRed.PuzzleSpotRed")
          (Components|StaticMesh|SetStaticMesh (Variables|/Game/Blueprints/SpherePuzzle/BP_PuzzleGun.BP_PuzzleGun_C|GetSplineMesh (Variables|Default|GetGun)) "/Game/0Mesh/Lasers/LaserPointerMesh_Red.LaserPointerMesh_Red")
          (Variables|/Game/Blueprints/SpherePuzzle/BP_SpherePuzzle.BP_SpherePuzzle_C|SetNowColor _puzzlesphere_4 (Variables|Default|GetColor) :!label _label)
          (Collision|SetCollisionEnabled (Variables|Default|GetSphereCollision) "NoCollision")
          (Variables|/Game/Blueprints/SpherePuzzle/BP_SpherePuzzle.BP_SpherePuzzle_C|SetNowSpot _puzzlesphere_4 self)
          (elif (Utilities|Enum|Equal(Enum) (Variables|Default|GetColor) (Utilities|Text|MakeLiteralText "Yellow"))
            (CallFunction|SetMaterial "/Game/0Mesh/PuzzleSpotYellow.PuzzleSpotYellow")
            (Components|StaticMesh|SetStaticMesh (Variables|/Game/Blueprints/SpherePuzzle/BP_PuzzleGun.BP_PuzzleGun_C|GetSplineMesh (Variables|Default|GetGun)) "/Game/0Mesh/Lasers/LaserPointerMesh_Yellow.LaserPointerMesh_Yellow")
            (goto _label)
            (elif (Utilities|Enum|Equal(Enum) (Variables|Default|GetColor) (Utilities|Text|MakeLiteralText "Green"))
              (CallFunction|SetMaterial "/Game/0Mesh/PuzzleSpotGreen.PuzzleSpotGreen")
              (Components|StaticMesh|SetStaticMesh (Variables|/Game/Blueprints/SpherePuzzle/BP_PuzzleGun.BP_PuzzleGun_C|GetSplineMesh (Variables|Default|GetGun)) "/Game/0Mesh/Lasers/LaserPointerMesh_Green.LaserPointerMesh_Green")
              (goto _label))))
        (elif (Utilities|Enum|Equal(Enum) (Variables|/Game/Blueprints/SpherePuzzle/BP_SpherePuzzle.BP_SpherePuzzle_C|GetNowColor (Variables|Default|GetPuzzleSphere)) (Variables|Default|GetColor))
          (Variables|/Game/Blueprints/SpherePuzzle/BP_PuzzleGun.BP_PuzzleGun_C|SetColor (Variables|Default|GetGun) "")
          (CallFunction|SetMaterial (Variables|/Game/Blueprints/SpherePuzzle/BP_SpherePuzzle.BP_SpherePuzzle_C|GetNowSpot _puzzlesphere_2) "/Game/0Mesh/PuzzleSpotBlue.PuzzleSpotBlue")
          (CallFunction|SetMaterial "/Game/0Mesh/PuzzleSpotBlue.PuzzleSpotBlue")
          (Components|StaticMesh|SetStaticMesh (Variables|/Game/Blueprints/SpherePuzzle/BP_PuzzleGun.BP_PuzzleGun_C|GetSplineMesh (Variables|Default|GetGun)) "/Game/0Mesh/Lasers/LaserPointerMesh_Blue.LaserPointerMesh_Blue")
          (if (Utilities|Enum|Equal(Enum) (Variables|/Game/Blueprints/SpherePuzzle/BP_SpherePuzzle.BP_SpherePuzzle_C|GetNowColor (Variables|Default|GetPuzzleSphere)) (Utilities|Text|MakeLiteralText "Red"))
            (SplineMesh|SetStartandEnd _line_red (Math|Transform|InverseTransformLocation _returnvalue_2 (Transformation|GetActorLocation (Variables|/Game/Blueprints/SpherePuzzle/BP_SpherePuzzle.BP_SpherePuzzle_C|GetNowSpot (Variables|Default|GetPuzzleSphere)))) "0, 0, 0" (Math|Transform|InverseTransformLocation _returnvalue_2 (Transformation|GetActorLocation)) "0, 0, 0" true :!class /Script/Engine.SplineMeshComponent)
            (Components|StaticMesh|SetStaticMesh _line_red "/Game/0Mesh/Lasers/LaserPointerMesh_Blue.LaserPointerMesh_Blue")
            (Variables|/Game/Blueprints/SpherePuzzle/BP_SpherePuzzle.BP_SpherePuzzle_C|SetRedOver _puzzlesphere_3 true)
            (Variables|/Game/Blueprints/SpherePuzzle/BP_SpherePuzzle.BP_SpherePuzzle_C|SetNowColor _puzzlesphere_2 "" :!label _label_2)
            (Collision|SetCollisionEnabled (Variables|Default|GetSphereCollision) "NoCollision")
            (bind _asbp_sphere_puzzle (Utilities|Casting|CastToBP_SpherePuzzle (Variables|Default|GetPuzzleSphere)))
            (Variables|/Game/Blueprints/SpherePuzzle/BP_SpherePuzzle.BP_SpherePuzzle_C|SetNowSpot _asbp_sphere_puzzle 0)
            (elif (Utilities|Enum|Equal(Enum) (Variables|/Game/Blueprints/SpherePuzzle/BP_SpherePuzzle.BP_SpherePuzzle_C|GetNowColor (Variables|Default|GetPuzzleSphere)) (Utilities|Text|MakeLiteralText "Yellow"))
              (SplineMesh|SetStartandEnd _line_yellow (Math|Transform|InverseTransformLocation _returnvalue_3 (Transformation|GetActorLocation (Variables|/Game/Blueprints/SpherePuzzle/BP_SpherePuzzle.BP_SpherePuzzle_C|GetNowSpot (Variables|Default|GetPuzzleSphere)))) "0, 0, 0" (Math|Transform|InverseTransformLocation _returnvalue_3 (Transformation|GetActorLocation)) "0, 0, 0" true :!class /Script/Engine.SplineMeshComponent)
              (Components|StaticMesh|SetStaticMesh _line_yellow "/Game/0Mesh/Lasers/LaserPointerMesh_Blue.LaserPointerMesh_Blue")
              (Variables|/Game/Blueprints/SpherePuzzle/BP_SpherePuzzle.BP_SpherePuzzle_C|SetYellowOver _puzzlesphere_3 true)
              (goto _label_2)
              (elif (Utilities|Enum|Equal(Enum) (Variables|/Game/Blueprints/SpherePuzzle/BP_SpherePuzzle.BP_SpherePuzzle_C|GetNowColor (Variables|Default|GetPuzzleSphere)) (Utilities|Text|MakeLiteralText "Green"))
                (SplineMesh|SetStartandEnd _line_green (Math|Transform|InverseTransformLocation _returnvalue (Transformation|GetActorLocation (Variables|/Game/Blueprints/SpherePuzzle/BP_SpherePuzzle.BP_SpherePuzzle_C|GetNowSpot (Variables|Default|GetPuzzleSphere)))) "0, 0, 0" (Math|Transform|InverseTransformLocation _returnvalue (Transformation|GetActorLocation)) "0, 0, 0" true :!class /Script/Engine.SplineMeshComponent)
                (Components|StaticMesh|SetStaticMesh _line_green "/Game/0Mesh/Lasers/LaserPointerMesh_Blue.LaserPointerMesh_Blue")
                (Variables|/Game/Blueprints/SpherePuzzle/BP_SpherePuzzle.BP_SpherePuzzle_C|SetGreenOver _puzzlesphere_3 true)
                (goto _label_2))))
          (else
            (CallFunction|SetMaterial (Variables|/Game/Blueprints/SpherePuzzle/BP_SpherePuzzle.BP_SpherePuzzle_C|GetNowSpot _puzzlesphere_2) "/Game/0Mesh/PuzzleSpotWhite.PuzzleSpotWhite")
            (Variables|/Game/Blueprints/SpherePuzzle/BP_SpherePuzzle.BP_SpherePuzzle_C|SetNowColor _puzzlesphere_2 "")
            (Variables|/Game/Blueprints/SpherePuzzle/BP_PuzzleGun.BP_PuzzleGun_C|SetColor (Variables|Default|GetGun) "")
            (Collision|SetCollisionEnabled (Variables|BP_PuzzleSpot_C|GetSphereCollision (Variables|/Game/Blueprints/SpherePuzzle/BP_SpherePuzzle.BP_SpherePuzzle_C|GetNowSpot _puzzlesphere_2)) "QueryAndPhysics")
            (Components|StaticMesh|SetStaticMesh (Variables|/Game/Blueprints/SpherePuzzle/BP_PuzzleGun.BP_PuzzleGun_C|GetSplineMesh (Variables|Default|GetGun)) "/Game/0Mesh/Lasers/LaserPointerMesh_White.LaserPointerMesh_White")))))))

(event EventBeginPlay
  (EventDispatchers|BindEventtoStartPuzzle (Variables|Default|GetPuzzleSphere) (delegate Custom|PuzzleStart))
  (Variables|Default|SetInitialLocation (Transformation|GetActorLocation))
  (EventDispatchers|BindEventtoInteraction (delegate Custom|커스텀이벤트_1)))

(event EventTick
  (params (DeltaSeconds :type Float%20%28single-precision%29))
  (bind _gun (Variables|Default|GetGun))
  (bind _puzzlesphere (Variables|Default|GetPuzzleSphere))
  (bind _nowspot (Variables|/Game/Blueprints/SpherePuzzle/BP_SpherePuzzle.BP_SpherePuzzle_C|GetNowSpot _puzzlesphere))
  (Utilities|IsValid _gun
    (:Is%20Valid
      (Utilities|IsValid (Variables|/Game/Blueprints/SpherePuzzle/BP_SpherePuzzle.BP_SpherePuzzle_C|GetNowSpot (Variables|Default|GetPuzzleSphere))
        (:Is%20Valid
          (if (not (Variables|/Game/Blueprints/BP_Equipment.BP_Equipment_C|GetisUse _gun))
            (CallFunction|SetMaterial _nowspot "/Game/0Mesh/PuzzleSpotWhite.PuzzleSpotWhite")
            (Variables|/Game/Blueprints/SpherePuzzle/BP_SpherePuzzle.BP_SpherePuzzle_C|SetNowColor _puzzlesphere "")
            (Variables|/Game/Blueprints/SpherePuzzle/BP_PuzzleGun.BP_PuzzleGun_C|SetColor (Variables|Default|GetGun) "")
            (Collision|SetCollisionEnabled (Variables|BP_PuzzleSpot_C|GetSphereCollision _nowspot) "QueryAndPhysics")
            (Components|StaticMesh|SetStaticMesh (Variables|/Game/Blueprints/SpherePuzzle/BP_PuzzleGun.BP_PuzzleGun_C|GetSplineMesh (Variables|Default|GetGun)) "/Game/0Mesh/Lasers/LaserPointerMesh_White.LaserPointerMesh_White")))))))

(fn ConstructionScript
  (bind _returnvalue (Actor|GetParentActor))
  (CallFunction|SetMaterial (Variables|Default|GetMaterial))
  (Utilities|IsValid _returnvalue
    (:Is%20Valid
      (bind _asbp_sphere_puzzle (Utilities|Casting|CastToBP_SpherePuzzle _returnvalue))
      (Variables|Default|SetPuzzleSphere _asbp_sphere_puzzle))))

(fn SetMaterial
  (params (Material :type Material%20Interface%20Object%20Reference))
  (Rendering|Material|SetMaterial (Variables|Default|GetPlane) 0 Material))