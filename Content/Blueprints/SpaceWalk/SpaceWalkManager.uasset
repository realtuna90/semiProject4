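; SpaceWalkManager runs the VR space walk stage as a linear task chain: button press, pipe throwaway, pipe repair, valve clear.
; On BeginPlay it hooks game mode stage changes, waits for a valid Button, then triggers a stage change.
; Each step increments a Task counter, with zero-delay polling loops binding the next event; repair also flags the valve.
; After the last task it pauses, changes stage and swaps streamed levels.
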(event Custom|repair
  (Math|Integer|IncrementInt (Variables|Default|GetTask)
    (:%20%20
      (Variables|/Game/Blueprints/SpaceWalk/BP_Valve.BP_Valve_C|SetIsRepaired (Variables|Default|GetValve) true))))

(event Custom|StageClear
  ;[1 1 1] 스테이지 클리어
  (bind _asvrgame_mode (Utilities|Casting|CastToVRGameMode (Game|GetGameMode)))
  (Default|StageChange _asvrgame_mode (Variables|Default|GetstageNum)))

(event Custom|StageStart
  (params (curStage :type LevelEnum%20Enum :default "NewEnumerator4"))
  (bind _pipebase (Variables|Default|GetPipeBase))
  (if (Utilities|Enum|Equal(Enum) curStage (Variables|Default|GetstageNum))
    (bind _asvrgame_mode (Utilities|Casting|CastToVRGameMode (Game|GetGameMode)))
    (Default|CallOnChangePhase _asvrgame_mode (Variables|Default|GetstageNum) (Variables|Default|GetPhase))
    (Utilities|FlowControl|Sequence
      (:then_0
        (if (== (Variables|Default|GetTask) 1) :!label _label
          (EventDispatchers|BindEventtoThrowaway _pipebase (delegate Custom|Clear))
          (else
            (Utilities|FlowControl|Delay 0.0)
            (goto _label))))
      (:then_1
        (if (== (Variables|Default|GetTask) 2) :!label _label_2
          (EventDispatchers|BindEventtoRepairComplete _pipebase (delegate Custom|repair))
          (else
            (Utilities|FlowControl|Delay 0.0)
            (goto _label_2))))
      (:then_2
        (if (== (Variables|Default|GetTask) 3) :!label _label_3
          (EventDispatchers|BindEventtoClear (Variables|Default|GetValve) (delegate Custom|Explode))
          (else
            (Utilities|FlowControl|Delay 0.0)
            (goto _label_3))))
      (:then_3
        (if (== (Variables|Default|GetTask) 4) :!label _label_4
          (Utilities|FlowControl|Delay 5.0)
          (bind _asvrgame_mode_2 (Utilities|Casting|CastToVRGameMode (Game|GetGameMode)))
          (CallFunction|StageClear)
          (Default|LoadLevel _asvrgame_mode_2 "SemiLevel_open_2" "outside_3")
          (else
            (Utilities|FlowControl|Delay 0.0)
            (goto _label_4)))))))

(event Custom|Explode
  (Math|Integer|IncrementInt (Variables|Default|GetTask)))

(event Custom|Clear
  (Math|Integer|IncrementInt (Variables|Default|GetTask)))

(event EventBeginPlay
  (bind _button (Variables|Default|Getbutton))
  (bind _asvrgame_mode (Utilities|Casting|CastToVRGameMode (Game|GetGameMode)))
  (EventDispatchers|BindEventtoOnChangeStage _asvrgame_mode (delegate Custom|StageStart))
  (Utilities|IsValid _button :!label _label
    (:Is%20Valid
      (EventDispatchers|BindEventtoPressed _button (delegate Custom|Clear))
      (Default|CallOnChangeStage _asvrgame_mode "NewEnumerator1"))
    (:Is%20Not%20Valid
      (Utilities|FlowControl|Delay 0.0)
      (goto _label))))

(fn ConstructionScript)