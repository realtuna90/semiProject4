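; Grabbable spare pipe for the SpaceWalk content that repairs a referenced PipeBase when dropped in its repair zone.
; Pickup turns off mesh physics and attaches it to the supplied component; Drop elsewhere restores physics and detaches.
; Dropping inside Repaircheck reveals PipeHide, destroys the spare and calls Repair.
; Tick polls the Box overlap to toggle a highlight material, while the begin/end overlap handlers have no effect.
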(event OnComponentBeginOverlap(Box)
  (params (OverlappedComponent :type Primitive%20Component%20Object%20Reference) (OtherActor :type Actor%20Object%20Reference) (OtherComp :type Primitive%20Component%20Object%20Reference) (OtherBodyIndex :type Integer) (bFromSweep :type Boolean) (SweepResult :type Hit%20Result%20Structure%20%28by%20ref%29))
  (if (== OverlappedComponent (Variables|/Game/Blueprints/SpaceWalk/BP_PipeBase.BP_PipeBase_C|GetRepaircheck (Variables|Default|GetPipeBase)))
    _))

(event OnComponentEndOverlap(Box)
  (params (OverlappedComponent :type Primitive%20Component%20Object%20Reference) (OtherActor :type Actor%20Object%20Reference) (OtherComp :type Primitive%20Component%20Object%20Reference) (OtherBodyIndex :type Integer))
  (if (== OverlappedComponent (Variables|/Game/Blueprints/SpaceWalk/BP_PipeBase.BP_PipeBase_C|GetRepaircheck (Variables|Default|GetPipeBase)))
    _))

(event EventPickup
  (params (AttachTo :type Scene%20Component%20Object%20Reference) (MotionController :type BP%20Motion%20Controller%20Object%20Reference))
  (bind _staticmesh (Variables|Default|GetStaticMesh))
  (Physics|SetSimulatePhysics _staticmesh false)
  (Transformation|AttachComponentToComponent _staticmesh AttachTo "None" "KeepWorld" "KeepWorld" "KeepWorld" false))

(event EventTick
  (params (DeltaSeconds :type Float%20%28single-precision%29))
  (if (Utilities|Array|ContainsItem (Class|PrimitiveComponent|GetOverlappingComponents (Variables|Default|GetBox)) (Variables|/Game/Blueprints/SpaceWalk/BP_PipeBase.BP_PipeBase_C|GetRepaircheck (Variables|Default|GetPipeBase)))
    (Rendering|Material|SetMaterial (Variables|Default|GetStaticMesh) 0 "/Game/M_MasterSciFiPopulateINST_Highlight.M_MasterSciFiPopulateINST_Highlight")
    (else
      (Rendering|Material|SetMaterial (Variables|Default|GetStaticMesh) 0 "/Game/SciFiPopulate/Materials/M_MasterSciFiPopulateINST.M_MasterSciFiPopulateINST"))))

(event EventDrop
  (bind _pipebase (Variables|Default|GetPipeBase))
  (if (Utilities|Array|ContainsItem (Class|PrimitiveComponent|GetOverlappingComponents (Variables|Default|GetBox)) (Variables|/Game/Blueprints/SpaceWalk/BP_PipeBase.BP_PipeBase_C|GetRepaircheck _pipebase))
    (Rendering|SetVisibility (Variables|/Game/Blueprints/SpaceWalk/BP_PipeBase.BP_PipeBase_C|GetPipeHide _pipebase) true false)
    (Actor|DestroyActor)
    (Default|Repair (Variables|Default|GetPipeBase))
    (else
      (Physics|SetSimulatePhysics (Variables|Default|GetStaticMesh) true)
      (Transformation|DetachFromActor "KeepWorld" "KeepWorld" "KeepWorld"))))

(fn ConstructionScript)