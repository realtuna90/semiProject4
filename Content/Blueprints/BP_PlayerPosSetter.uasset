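; BP_PlayerPosSetter is a placed marker actor that moves the player pawn to its own location and rotation when the game reaches its assigned stage.
; On BeginPlay it binds to the VRGameMode stage-change event.
; When the new stage matches its Stage variable and is Stage 0, 1 or 2, it repositions player pawn 0 without sweep and prints a debug message.
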(event Custom|PlayerSetting
  (params (curStage :type LevelEnum%20Enum :default "NewEnumerator4"))
  (bind _returnvalue (Game|Player|GetPlayerPawn 0))
  (if (Utilities|Enum|Equal(Enum) curStage (Variables|Default|GetStage))
    (switch Utilities|FlowControl|Switch|SwitchonLevelEnum curStage
      (:NewEnumerator3
        _)
      (:NewEnumerator0
        _)
      (:NewEnumerator1
        _))
    (Transformation|SetActorLocation _returnvalue (Transformation|GetActorLocation) false false)
    (Transformation|SetActorRotation _returnvalue (Transformation|GetActorRotation))
    (Development|PrintString "LocationSetting Seccess" true true "(R=0.000000,G=0.660000,B=1.000000,A=1.000000)" 5.0)))

(event EventBeginPlay
  (bind _asvrgame_mode (Utilities|Casting|CastToVRGameMode (Game|GetGameMode)))
  (EventDispatchers|BindEventtoOnChangeStage _asvrgame_mode (delegate Custom|PlayerSetting)))

(fn ConstructionScript)