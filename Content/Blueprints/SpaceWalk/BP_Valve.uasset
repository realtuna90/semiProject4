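; VR valve for the SpaceWalk sequence that the player grabs and twists to control pipe smoke, registering itself with SpaceWalkManager.
; While held, Tick applies yaw deltas from the hand's right vector, projected on the valve's plane, within soft rotation limits.
; The upper limit stops BP_Pipe smoking and backing off restarts it, while audio volume follows rotation.
; Once repaired, reaching the lower limit triggers a one-time explosion that knocks the pawn backward.
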(event EventBeginPlay
  (bind _returnvalue (Actor|GetActorOfClass "/Game/Blueprints/SpaceWalk/SpaceWalkManager.SpaceWalkManager_C"))
  (Variables|/Game/Blueprints/SpaceWalk/SpaceWalkManager.SpaceWalkManager_C|SetValve _returnvalue self))

(event EventTick
  (params (DeltaSeconds :type Float%20%28single-precision%29))
  (Utilities|FlowControl|Sequence
    (:then_0
      (if (Variables|Default|GetIsUse)
        (if (<= (Variables|Default|GetRotateValue) -5e+01)
          (if (>= (.Yaw (Math|Rotator|BreakRotator (Math|Rotator|Delta(Rotator) (Math|Rotator|FindLookatRotation (Math|Vector|MakeVector 0.0 0.0 0.0) (Math|Vector|Normalize (Math|Vector|ProjectVectorontoPlane (Math|Vector|GetRightVector (Variables|/Game/Blueprints/BP_MotionController.BP_MotionController_C|GetHandMesh (stale EventPickup MotionController))) (Transformation|GetActorUpVector)))) (Variables|Default|GetNowRotation)))) 0.0)
            (Transformation|AddRelativeRotation (Variables|Default|GetStaticMesh) (Math|Rotator|Delta(Rotator) (Math|Rotator|FindLookatRotation (Math|Vector|MakeVector 0.0 0.0 0.0) (Math|Vector|Normalize (Math|Vector|ProjectVectorontoPlane (Math|Vector|GetRightVector (Variables|/Game/Blueprints/BP_MotionController.BP_MotionController_C|GetHandMesh (stale EventPickup MotionController))) (Transformation|GetActorUpVector)))) (Variables|Default|GetNowRotation)) false false :!label _label)
            (Variables|Default|SetRotateValue (+ (.Yaw (Math|Rotator|BreakRotator (Math|Rotator|Delta(Rotator) (Math|Rotator|FindLookatRotation (Math|Vector|MakeVector 0.0 0.0 0.0) (Math|Vector|Normalize (Math|Vector|ProjectVectorontoPlane (Math|Vector|GetRightVector (Variables|/Game/Blueprints/BP_MotionController.BP_MotionController_C|GetHandMesh (stale EventPickup MotionController))) (Transformation|GetActorUpVector)))) (Variables|Default|GetNowRotation)))) (Variables|Default|GetRotateValue)))
            (Variables|Default|SetNowRotation (Math|Rotator|FindLookatRotation (Math|Vector|MakeVector 0.0 0.0 0.0) (Math|Vector|Normalize (Math|Vector|ProjectVectorontoPlane (Math|Vector|GetRightVector (Variables|/Game/Blueprints/BP_MotionController.BP_MotionController_C|GetHandMesh (stale EventPickup MotionController))) (Transformation|GetActorUpVector))))))
          (elif (>= (Variables|Default|GetRotateValue) 2.5e+02)
            (if (<= (.Yaw (Math|Rotator|BreakRotator (Math|Rotator|Delta(Rotator) (Math|Rotator|FindLookatRotation (Math|Vector|MakeVector 0.0 0.0 0.0) (Math|Vector|Normalize (Math|Vector|ProjectVectorontoPlane (Math|Vector|GetRightVector (Variables|/Game/Blueprints/BP_MotionController.BP_MotionController_C|GetHandMesh (stale EventPickup MotionController))) (Transformation|GetActorUpVector)))) (Variables|Default|GetNowRotation)))) 0.0)
              (goto _label))
            (else
              (goto _label))))))
    (:then_1
      (if (>= (Variables|Default|GetRotateValue) 2.5e+02)
        (Utilities|FlowControl|DoOnce false :!label _label_2
          (:Completed
            (bind _returnvalue (Actor|GetActorOfClass "/Game/Blueprints/SpaceWalk/BP_Pipe.BP_Pipe_C"))
            (Variables|/Game/Blueprints/SpaceWalk/BP_Pipe.BP_Pipe_C|SetIsSmoking _returnvalue false)
            (goto _label_3 Reset)))
        (else
          (Utilities|FlowControl|DoOnce false :!label _label_3
            (:Completed
              (bind _returnvalue_2 (Actor|GetActorOfClass "/Game/Blueprints/SpaceWalk/BP_Pipe.BP_Pipe_C"))
              (Variables|/Game/Blueprints/SpaceWalk/BP_Pipe.BP_Pipe_C|SetIsSmoking _returnvalue_2 true)
              (goto _label_2 Reset))))))
    (:then_2
      (if (Variables|Default|GetIsRepaired)
        (if (<= (Variables|Default|GetRotateValue) -5e+01)
          (Utilities|FlowControl|DoOnce false
            (:Completed
              (Default|CallExplode)
              (bind _asmotion_controller_pawn (Utilities|Casting|CastToMotionControllerPawn (Game|Player|GetPlayerPawn 0)))
              (Physics|AddImpulseatLocation (Variables|/Game/Blueprints/MotionControllerPawn.MotionControllerPawn_C|GetPhysicsRoot _asmotion_controller_pawn) (* (Math|Vector|GetForwardVector (Variables|/Game/Blueprints/MotionControllerPawn.MotionControllerPawn_C|GetPhysicsRoot _asmotion_controller_pawn)) -5e+02) (Transformation|GetWorldLocation (Variables|/Game/Blueprints/MotionControllerPawn.MotionControllerPawn_C|GetPhysicsRoot _asmotion_controller_pawn)) "None")
              (Class|PrimitiveComponent|SetLinearDamping (Variables|/Game/Blueprints/MotionControllerPawn.MotionControllerPawn_C|GetPhysicsRoot _asmotion_controller_pawn) 2.0)
              (Utilities|FlowControl|Delay 2.0)
              (Class|PrimitiveComponent|SetLinearDamping (Variables|/Game/Blueprints/MotionControllerPawn.MotionControllerPawn_C|GetPhysicsRoot _asmotion_controller_pawn) 0.0))))))
    (:then_3
      (Audio|Components|Audio|SetVolumeMultiplier (Variables|Default|GetAudio) (+ (* (Variables|Default|GetRotateValue) -0.01) 2.5) :!class /Script/Engine.AudioComponent))))

(event EventPickup
  (params (AttachTo :type Scene%20Component%20Object%20Reference) (MotionController :type BP%20Motion%20Controller%20Object%20Reference))
  (Variables|Default|SetIsUse true)
  (Variables|Default|SetNowRotation (Math|Rotator|FindLookatRotation (Math|Vector|MakeVector 0.0 0.0 0.0) (Math|Vector|Normalize (Math|Vector|ProjectVectorontoPlane (Math|Vector|GetRightVector (Variables|/Game/Blueprints/BP_MotionController.BP_MotionController_C|GetHandMesh MotionController)) (Transformation|GetActorUpVector))))))

(event EventDrop
  (Variables|Default|SetIsUse false))

(fn ConstructionScript)