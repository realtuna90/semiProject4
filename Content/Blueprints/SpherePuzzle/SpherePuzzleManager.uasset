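; Stage manager for the sphere puzzle that tracks clear signals and calls the VR game mode's StageChange.
; On BeginPlay it binds to stage changes, then polls until Puzzle, Lever and Button are valid, routing their events into one Clear flag.
; On its stage, three zero-delay polling branches start together, each consuming that flag to print, reveal the puzzle, or complete the stage.
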(event Custom|Clear
  (Variables|Default|SetClear? true))

(event Custom|StageClear
  ;[1 1 1] 스테이지 클리어
  (bind _asvrgame_mode (Utilities|Casting|CastToVRGameMode (Game|GetGameMode)))
  (Default|StageChange _asvrgame_mode (Variables|Default|GetstageNum)))

(event Custom|StageStart
  (params (curStage :type LevelEnum%20Enum :default "NewEnumerator3"))
  (Development|PrintString "Hello" true true "(R=0.000000,G=0.660000,B=1.000000,A=1.000000)" 3e+01)
  (if (Utilities|Enum|Equal(Enum) curStage (Variables|Default|GetstageNum))
    (Utilities|FlowControl|Sequence
      (:then_0
        (Variables|Default|SetClear? false)
        (if (Variables|Default|GetClear?) :!label _label
          (Variables|Default|SetClear? false)
          (Development|PrintString "Hello" true true "(R=0.000000,G=0.660000,B=1.000000,A=1.000000)" 1e+01)
          (else
            (Utilities|FlowControl|Delay 0.0)
            (goto _label))))
      (:then_1
        (Variables|Default|SetClear? false)
        (if (Variables|Default|GetClear?) :!label _label_2
          (Variables|Default|SetClear? false)
          (Rendering|SetActorHiddenInGame (Variables|Default|GetPuzzle) false)
          (Development|PrintString "Hello" true true "(R=0.000000,G=0.660000,B=1.000000,A=1.000000)" 1e+01)
          (else
            (Utilities|FlowControl|Delay 0.0)
            (goto _label_2))))
      (:then_2
        (Variables|Default|SetClear? false)
        (if (Variables|Default|GetClear?) :!label _label_3
          (Variables|Default|SetClear? false)
          (Development|PrintString "CLEAR!!!" true true "(R=0.000000,G=0.660000,B=1.000000,A=1.000000)" 3e+01)
          (CallFunction|StageClear)
          (else
            (Utilities|FlowControl|Delay 0.0)
            (goto _label_3)))))))

(event EventBeginPlay
  (bind _puzzle (Variables|Default|GetPuzzle))
  (bind _lever (Variables|Default|GetLever))
  (bind _button (Variables|Default|Getbutton))
  (bind _asvrgame_mode (Utilities|Casting|CastToVRGameMode (Game|GetGameMode)))
  (EventDispatchers|BindEventtoOnChangeStage _asvrgame_mode (delegate Custom|StageStart))
  (Utilities|IsValid _puzzle :!label _label
    (:Is%20Valid
      (EventDispatchers|BindEventtoClearPuzzle _puzzle (delegate Custom|Clear))
      (Utilities|IsValid _lever :!label _label_2
        (:Is%20Valid
          (EventDispatchers|BindEventtoLeverInput _lever (delegate Custom|Clear))
          (Utilities|IsValid _button :!label _label_3
            (:Is%20Valid
              (EventDispatchers|BindEventtoPressed _button (delegate Custom|Clear)))
            (:Is%20Not%20Valid
              (Utilities|FlowControl|Delay 0.0)
              (goto _label_3))))
        (:Is%20Not%20Valid
          (Utilities|FlowControl|Delay 0.0)
          (goto _label_2))))
    (:Is%20Not%20Valid
      (Utilities|FlowControl|Delay 0.0)
      (goto _label))))

(fn ConstructionScript)