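; BP_ClosePanel is a screwed-down panel that the player can pick up and drop only after all its screws are out.
; On BeginPlay it registers itself with its child BP_Screw actors and counts them.
; ScrewOut tallies fully pulled screws and sets Movable when all are out.
; Pickup then disables physics and attaches the panel, Drop reverses this, and ScrewHighLightOff clears every screw highlight.
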(event EventPickup
  (params (AttachTo :type Scene%20Component%20Object%20Reference) (MotionController :type BP%20Motion%20Controller%20Object%20Reference))
  (if (Variables|Default|GetMovable)
    (Physics|SetSimulatePhysics (Variables|Default|GetClosePanel) false)
    (Transformation|AttachComponentToComponent (VehicleSound|GetRootComponent) AttachTo "None" "KeepWorld" "KeepWorld" "KeepWorld" false)))

(event EventDrop
  (if (Variables|Default|GetMovable)
    (Physics|SetSimulatePhysics (Variables|Default|GetClosePanel) true)
    (Transformation|DetachFromActor "KeepWorld" "KeepWorld" "KeepWorld")))

(event EventBeginPlay
  (for _array_element (Actor|GetAllChildActors true)
    (bind _asbp_screw (Utilities|Casting|CastToBP_Screw _array_element))
    (Variables|/Game/Blueprints/BP_Screw.BP_Screw_C|SetPanelActor _asbp_screw self)
    (Utilities|Array|Insert (Variables|Default|GetScrews) _asbp_screw (Variables|Default|GetarrayCount))
    (bind _result (Math|Integer|IncrementInt (Variables|Default|GetarrayCount))
      (:%20%20
        (Variables|Default|SetMaxCount _result)))))

(fn ConstructionScript)

(fn ScrewOut
  (params (Nasa :type BP%20Screw%20Object%20Reference))
  (if (Variables|/Game/Blueprints/BP_Screw.BP_Screw_C|GetPullOutOver Nasa)
    (bind _result (Math|Integer|IncrementInt (Variables|Default|GetCount))
      (:%20%20
        (Variables|Default|SetCount _result)
        (if (== (Variables|Default|GetCount) (Variables|Default|GetMaxCount))
          (Variables|Default|SetMovable true))))))

(fn ScrewHighLightOff
  (for _array_element (Variables|Default|GetScrews)
    (Default|HighLightOff (Variables|/Game/Blueprints/BP_Screw.BP_Screw_C|GetHighLight _array_element))))