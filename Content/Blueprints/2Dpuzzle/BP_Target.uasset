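; Laser target for the 2D puzzle that clears when lit from both left and right while active.
; Left and right hit events set per-side flags that pick the mesh material and TargetClear state.
; When both are set, it highlights and calls Check on the parent BP_2DPuzzle.
; Tick resets both flags and the idle material, so hits must repeat every frame, but leaves TargetClear untouched.
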(event Custom|RightOn
  (if (Variables|Default|GetIsActivate)
    (Variables|Default|SetRightLaser true)
    (if (Variables|Default|GetLeftLaser)
      (Rendering|Material|SetMaterial (Variables|Default|GetStaticMesh) 0 "/Engine/MapTemplates/Materials/BasicAsset01.BasicAsset01")
      (if (Variables|Default|GetRightLaser)
        (Rendering|Material|SetMaterial (Variables|Default|GetStaticMesh) 0 "/Game/VirtualReality/Materials/BasicHighlightMaterial.BasicHighlightMaterial")
        (Variables|Default|SetTargetClear true)
        (bind _asbp_2dpuzzle (Utilities|Casting|CastToBP_2DPuzzle (Actor|GetParentActor)))
        (Default|Check _asbp_2dpuzzle)
        (else
          (Variables|Default|SetTargetClear false)))
      (elif (Variables|Default|GetRightLaser)
        (Rendering|Material|SetMaterial (Variables|Default|GetStaticMesh) 0 "/Game/2Materials/BasicAsset03.BasicAsset03")
        (Variables|Default|SetTargetClear false)))))

(event Custom|LeftOn
  (bind _rightlaser (Variables|Default|GetRightLaser))
  (if (Variables|Default|GetIsActivate)
    (Variables|Default|SetLeftLaser true)
    (if (Variables|Default|GetLeftLaser)
      (Rendering|Material|SetMaterial (Variables|Default|GetStaticMesh) 0 "/Engine/MapTemplates/Materials/BasicAsset01.BasicAsset01")
      (if _rightlaser
        (Rendering|Material|SetMaterial (Variables|Default|GetStaticMesh) 0 "/Game/VirtualReality/Materials/BasicHighlightMaterial.BasicHighlightMaterial")
        (Variables|Default|SetTargetClear true)
        (bind _asbp_2dpuzzle (Utilities|Casting|CastToBP_2DPuzzle (Actor|GetParentActor)))
        (Default|Check _asbp_2dpuzzle)
        (else
          (Variables|Default|SetTargetClear false)))
      (elif _rightlaser
        (Rendering|Material|SetMaterial (Variables|Default|GetStaticMesh) 0 "/Game/2Materials/BasicAsset03.BasicAsset03")
        (Variables|Default|SetTargetClear false)))))

(event EventTick
  (params (DeltaSeconds :type Float%20%28single-precision%29))
  (Variables|Default|SetLeftLaser false)
  (Variables|Default|SetRightLaser false)
  (Rendering|Material|SetMaterial (Variables|Default|GetStaticMesh) 0 "/Engine/MapTemplates/Materials/BasicAsset02.BasicAsset02"))

(event EventBeginPlay
  (EventDispatchers|BindEventtoLeftHit (delegate Custom|LeftOn))
  (EventDispatchers|BindEventtoRightHit (delegate Custom|RightOn)))

(fn ConstructionScript)