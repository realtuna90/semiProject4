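; Component that marks its owning actor with an arrow highlight during a given stage and phase of the VR game.
; It listens to VRGameMode's phase-change event, showing the blue arrow when stage and phase match its own and hiding it otherwise.
; HighLightOn spawns BP_HighLight2 once and reuses it, setting arm length and a red material when accented.
; Tick copies the owner's location and rotation to the spawned highlight instead of attaching it.
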(event Custom|OnChangePhase
  (params (Stage :type LevelEnum%20Enum :default "NewEnumerator4") (Phase :type Integer))
  (if (and (Utilities|Enum|Equal(Enum) Stage (Variables|Default|GetStage)) (== Phase (Variables|Default|GetPhase)))
    (CallFunction|HighLighton false)
    (else
      (CallFunction|HighLightOff))))

(event EventBeginPlay
  (Utilities|FlowControl|Sequence
    (:then_1
      (bind _asvrgame_mode (Utilities|Casting|CastToVRGameMode (Game|GetGameMode)))
      (EventDispatchers|BindEventtoOnChangePhase _asvrgame_mode (delegate Custom|OnChangePhase)))))

(event EventTick
  (params (DeltaSeconds :type Float%20%28single-precision%29))
  (bind _returnvalue (Components|GetOwner))
  (bind _object (Variables|Default|GetObject))
  (bind _returnvalue_2 (Transformation|GetActorTransform _returnvalue))
  (Utilities|IsValid (Variables|Default|GetObject)
    (:Is%20Valid
      (Transformation|SetActorLocation _object (.location _returnvalue_2) false false)
      (Transformation|SetActorRotation _object (.rotation _returnvalue_2)))))

(fn HighLighton
  (params (accent :type Boolean))
  (bind _returnvalue (Components|GetOwner))
  (bind _returnvalue_2 (Transformation|GetActorTransform _returnvalue))
  (Utilities|IsValid (Variables|Default|GetObject)
    (:Is%20Valid
      (Rendering|SetActorHiddenInGame (Variables|Default|GetObject) false))
    (:Is%20Not%20Valid
      (bind _returnvalue_3 (Game|SpawnActorfromClass "/Game/Blueprints/BP_HighLight2.BP_HighLight2_C" (Math|Transform|MakeTransform (.location _returnvalue_2) (.rotation _returnvalue_2) "0.100000,0.100000,0.100000") "AlwaysSpawn" 0 0))
      (Variables|Default|SetObject _returnvalue_3)))
  (if accent
    (Rendering|Material|SetMaterial (Variables|/Game/Blueprints/BP_HighLight2.BP_HighLight2_C|GetArrowMesh (Variables|Default|GetObject)) 0 "/Game/2Materials/M_RedHighLight.M_RedHighLight")
    (else
      (Rendering|Material|SetMaterial (Variables|/Game/Blueprints/BP_HighLight2.BP_HighLight2_C|GetArrowMesh (Variables|Default|GetObject)) 0 "/Game/2Materials/M_BlueHighLight.M_BlueHighLight")))
  (Rendering|SetVisibility (Variables|/Game/Blueprints/BP_HighLight2.BP_HighLight2_C|GetArrowMesh (Variables|Default|GetObject)) true false)
  (Variables|/Script/Engine.SpringArmComponent|SetTargetArmLength (Variables|/Game/Blueprints/BP_HighLight2.BP_HighLight2_C|GetSpringArm (Variables|Default|GetObject)) (Variables|Default|GetArmLength)))

(fn HighLightOff
  (bind _object (Variables|Default|GetObject))
  (Utilities|IsValid _object
    (:Is%20Valid
      (Rendering|SetVisibility (Variables|/Game/Blueprints/BP_HighLight2.BP_HighLight2_C|GetArrowMesh _object) false false))))