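; BP_GasManager manages the gas room stage, keyed to its StageNum in VRGameMode.
; On BeginPlay it binds to the game mode's stage-change event, then finds and hides BP_GasRoom.
; When its stage starts it reveals the room and runs a Clear-flag polling loop, which exits at once because Clear is preset true.
; A separate StageClear event passes StageNum to the game mode's StageChange, but nothing here calls it.
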(event Custom|StageClear
  ;[1 1 1] 스테이지 클리어
  (bind _asvrgame_mode (Utilities|Casting|CastToVRGameMode (Game|GetGameMode)))
  (Default|StageChange _asvrgame_mode (Variables|Default|GetstageNum)))

(event Custom|StageStart
  (params (curStage :type LevelEnum%20Enum :default "NewEnumerator4"))
  (if (Utilities|Enum|Equal(Enum) curStage (Variables|Default|GetstageNum))
    (Utilities|FlowControl|Sequence
      (:then_0
        (Rendering|SetActorHiddenInGame (Variables|Default|GetgasRoom) false)
        (Variables|Default|SetClear? true)
        (if (Variables|Default|GetClear?) :!label _label
          (Variables|Default|SetClear? false)
          (else
            (Utilities|FlowControl|Delay 0.0)
            (goto _label)))))))

(event EventBeginPlay
  (bind _asvrgame_mode (Utilities|Casting|CastToVRGameMode (Game|GetGameMode)))
  (EventDispatchers|BindEventtoOnChangeStage _asvrgame_mode (delegate Custom|StageStart))
  (bind _returnvalue (Actor|GetActorOfClass "/Game/Blueprints/GasEvent/BP_GasRoom.BP_GasRoom_C"))
  (bind _output_get (Variables|Default|SetgasRoom _returnvalue))
  (Rendering|SetActorHiddenInGame _output_get true))

(fn ConstructionScript)