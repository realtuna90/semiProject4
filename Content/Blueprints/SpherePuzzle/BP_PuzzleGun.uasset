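; Equippable laser gun for the sphere puzzle that draws colored lines from puzzle spots to wherever it is aimed.
; While used outside the sphere, Tick line-traces forward, stretches a spline-mesh beam, spawns spark particles and toggles spark sound on hit changes.
; Hit BP_PuzzleSpots set the active color and receive an interaction call.
; The parent BP_SpherePuzzle's matching red, yellow or green line then follows the hit point.
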(event EventTick
  (params (DeltaSeconds :type Float%20%28single-precision%29))
  (bind _tracepoint (Variables|Default|GetTracePoint))
  (bind _traceend (Variables|Default|GetTraceEnd))
  (bind _sparksound (Variables|Default|GetSparkSound))
  (bind _returnvalue (Transformation|GetWorldLocation _tracepoint))
  (if (Variables|Default|GetisEquipped)
    (if (Variables|Default|GetisUse)
      (if (Variables|Default|GetIsInSphere)
        (Rendering|SetVisibility (Variables|Default|GetSplineMesh) false false :!label _label)
        (Utilities|FlowControl|DoOnce false :!label _label_2
          (:Completed
            (Components|Activation|Deactivate (Variables|Default|GetSparkSound))
            (goto _label_4 Reset)))
        (else
          (Utilities|FlowControl|Sequence
            (:then_0
              (Variables|Default|SetonHit false)
              (bind _outhit (Collision|LineTraceByChannel _returnvalue (+ _returnvalue (* (Math|Vector|GetForwardVector (Transformation|GetWorldRotation _tracepoint)) 1e+03)) "TraceTypeQuery3" true 0 "None"))
              (bind _output_get (Variables|Default|SetonHit (.bBlockingHit (Collision|BreakHitResult _outhit))))
              (Transformation|SetWorldLocation _traceend (.Location (Collision|BreakHitResult _outhit)) false false)
              (SplineMesh|SetStartandEnd (Variables|Default|GetSplineMesh) (Variables|/Script/Engine.SceneComponent|GetRelativeLocation (Variables|Default|GetTracePoint)) "0, 0, 0" (Variables|/Script/Engine.SceneComponent|GetRelativeLocation _traceend) "0, 0, 0" _output_get :!class /Script/Engine.SplineMeshComponent)
              (Rendering|SetVisibility (Variables|Default|GetSplineMesh) true false)
              (Effects|SpawnEmitteratLocation "/Game/FX/P_DriverSpark.P_DriverSpark" (.Location (Collision|BreakHitResult _outhit)) "0, 0, 0" "0.100000,0.100000,0.100000" false)
              (if (Utilities|Text|TextIsEmpty (Variables|Default|GetColor))
                (bind _asbp_puzzle_spot (Utilities|Casting|CastToBP_PuzzleSpot (.HitActor (Collision|BreakHitResult _outhit)) :!label _label_3))
                (Variables|Default|SetColor (Variables|/Game/Blueprints/SpherePuzzle/BP_PuzzleSpot.BP_PuzzleSpot_C|GetColor _asbp_puzzle_spot))
                (Default|CallInteraction _asbp_puzzle_spot self)
                (Variables|Default|SetPuzzleSpot _asbp_puzzle_spot)
                (Utilities|FlowControl|DoOnce false
                  (:Completed
                    (bind _asbp_sphere_puzzle (Utilities|Casting|CastToBP_SpherePuzzle (Actor|GetParentActor _asbp_puzzle_spot)))
                    (Variables|Default|SetPuzzle _asbp_sphere_puzzle)))
                (elif (Utilities|Enum|Equal(Enum) (Variables|Default|GetColor) (Utilities|Text|MakeLiteralText "Red"))
                  (SplineMesh|SetStartandEnd (Variables|/Game/Blueprints/SpherePuzzle/BP_SpherePuzzle.BP_SpherePuzzle_C|GetLine_Red (Variables|Default|GetPuzzle)) (Math|Transform|InverseTransformLocation (Transformation|GetWorldTransform (Variables|/Game/Blueprints/SpherePuzzle/BP_SpherePuzzle.BP_SpherePuzzle_C|GetLine_Red (Variables|Default|GetPuzzle))) (.Location (Collision|BreakHitResult _outhit))) "0, 0, 0" (Math|Transform|InverseTransformLocation (Transformation|GetWorldTransform (Variables|/Game/Blueprints/SpherePuzzle/BP_SpherePuzzle.BP_SpherePuzzle_C|GetLine_Red (Variables|Default|GetPuzzle))) (Transformation|GetActorLocation (Variables|Default|GetPuzzleSpot))) "0, 0, 0" true :!class /Script/Engine.SplineMeshComponent)
                  (Rendering|SetVisibility (Variables|/Game/Blueprints/SpherePuzzle/BP_SpherePuzzle.BP_SpherePuzzle_C|GetLine_Red (Variables|Default|GetPuzzle)) true false)
                  (goto _label_3)
                  (elif (Utilities|Enum|Equal(Enum) (Variables|Default|GetColor) (Utilities|Text|MakeLiteralText "Yellow"))
                    (SplineMesh|SetStartandEnd (Variables|/Game/Blueprints/SpherePuzzle/BP_SpherePuzzle.BP_SpherePuzzle_C|GetLine_Yellow (Variables|Default|GetPuzzle)) (Math|Transform|InverseTransformLocation (Transformation|GetWorldTransform (Variables|/Game/Blueprints/SpherePuzzle/BP_SpherePuzzle.BP_SpherePuzzle_C|GetLine_Yellow (Variables|Default|GetPuzzle))) (.Location (Collision|BreakHitResult _outhit))) "0, 0, 0" (Math|Transform|InverseTransformLocation (Transformation|GetWorldTransform (Variables|/Game/Blueprints/SpherePuzzle/BP_SpherePuzzle.BP_SpherePuzzle_C|GetLine_Yellow (Variables|Default|GetPuzzle))) (Transformation|GetActorLocation (Variables|Default|GetPuzzleSpot))) "0, 0, 0" true :!class /Script/Engine.SplineMeshComponent)
                    (Rendering|SetVisibility (Variables|/Game/Blueprints/SpherePuzzle/BP_SpherePuzzle.BP_SpherePuzzle_C|GetLine_Yellow (Variables|Default|GetPuzzle)) true false)
                    (goto _label_3)
                    (elif (Utilities|Enum|Equal(Enum) (Variables|Default|GetColor) (Utilities|Text|MakeLiteralText "Green"))
                      (SplineMesh|SetStartandEnd (Variables|/Game/Blueprints/SpherePuzzle/BP_SpherePuzzle.BP_SpherePuzzle_C|GetLine_Green (Variables|Default|GetPuzzle)) (Math|Transform|InverseTransformLocation (Transformation|GetWorldTransform (Variables|/Game/Blueprints/SpherePuzzle/BP_SpherePuzzle.BP_SpherePuzzle_C|GetLine_Green (Variables|Default|GetPuzzle))) (.Location (Collision|BreakHitResult _outhit))) "0, 0, 0" (Math|Transform|InverseTransformLocation (Transformation|GetWorldTransform (Variables|/Game/Blueprints/SpherePuzzle/BP_SpherePuzzle.BP_SpherePuzzle_C|GetLine_Green (Variables|Default|GetPuzzle))) (Transformation|GetActorLocation (Variables|Default|GetPuzzleSpot))) "0, 0, 0" true :!class /Script/Engine.SplineMeshComponent)
                      (Rendering|SetVisibility (Variables|/Game/Blueprints/SpherePuzzle/BP_SpherePuzzle.BP_SpherePuzzle_C|GetLine_Green (Variables|Default|GetPuzzle)) true false)
                      (goto _label_3))))))
            (:then_1
              (if (Math|Boolean|Equal(Boolean) (Variables|Default|GetonHit) false)
                (CallFunction|Laseron)))
            (:then_2
              (if (Variables|Default|GetonHit)
                (Utilities|FlowControl|DoOnce false :!label _label_4
                  (:Completed
                    (Transformation|SetWorldLocation _sparksound (Transformation|GetWorldLocation (Variables|Default|GetTraceEnd)) false false)
                    (Components|Activation|Activate _sparksound false)
                    (goto _label_2 Reset)))
                (else
                  (goto _label_2)))))))
      (else
        (goto _label)))
    (else
      (goto _label_2))))

(fn ConstructionScript
  (Variables|Default|SetHighLightMesh 0))

(fn Laseron
  (bind _tracepoint (Variables|Default|GetTracePoint))
  (bind _splinemesh (Variables|Default|GetSplineMesh))
  (bind _relativelocation (Variables|/Script/Engine.SceneComponent|GetRelativeLocation _tracepoint))
  (SplineMesh|SetStartandEnd _splinemesh _relativelocation "0, 0, 0" (+ _relativelocation (* (Math|Vector|GetForwardVector (Variables|/Script/Engine.SceneComponent|GetRelativeRotation _tracepoint)) 1e+03)) "0, 0, 0" true :!class /Script/Engine.SplineMeshComponent)
  (Rendering|SetVisibility _splinemesh true false))